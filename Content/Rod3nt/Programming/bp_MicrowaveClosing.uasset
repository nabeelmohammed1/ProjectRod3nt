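; Microwave door trap that closes when something overlaps its box trigger and sends a "Microwave" achievement message through the game instance.
; A timeline vector, added to the door's rotation stored at BeginPlay, drives the actor's rotation.
; The same timeline update, on every tick, creates and plays the MicrowaveClosingRat level sequence, calls HudOffMessage on the player pawn, and disables input until a two-second delay ends.
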(event OnComponentBeginOverlap(Box)
  (params (OverlappedComponent :type Primitive%20Component%20Object%20Reference) (OtherActor :type Actor%20Object%20Reference) (OtherComp :type Primitive%20Component%20Object%20Reference) (OtherBodyIndex :type Integer) (bFromSweep :type Boolean) (SweepResult :type Hit%20Result%20Structure%20%28by%20ref%29))
  (CallFunction|CloseDoor)
  (Class|BIGI|AchievmentType(Message) (Game|GetGameInstance) "Microwave" 1.0))

(event Custom|CloseDoor
  (bind _returnvalue (Game|Player|GetPlayerPawn 0))
  (bind _returnvalue_2 (Game|GetPlayerController 0))
  (bind _vector (Timeline|Timeline Play)
    (:Update
      (Transformation|SetActorRotation (Math|Conversions|RotationFromXVector (+ (Variables|Default|GetNewVar) _vector)))
      (bind _outactor (Sequencer|Player|CreateLevelSequencePlayer "/Game/Rod3nt/DeathSequences/microwaveClosingRat.microwaveClosingRat"))
      (Class|BIPLayeRat|HudOff(Message) (Game|Player|GetPlayerPawn 0))
      (Sequencer|Player|Play (Variables|/Script/LevelSequence.LevelSequenceActor|GetSequencePlayer _outactor) :!class /Script/MovieScene.MovieSceneSequencePlayer)
      (Input|DisableInput _returnvalue _returnvalue_2)
      (Utilities|FlowControl|Delay 2.0)
      (Input|EnableInput _returnvalue _returnvalue_2))))

(event EventBeginPlay
  (Variables|Default|SetNewVar (Transformation|GetWorldRotation (Variables|Default|GetDoor))))

(fn ConstructionScript)