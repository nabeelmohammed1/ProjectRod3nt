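; Poison can hazard that releases a damaging poison cloud once it has been knocked over and comes to rest.
; Overlap by a BI_Physics actor starts mesh physics and a looping timer that polls velocity until it is near zero.
; At rest, it stops the timer, activates poison Niagara effects and enables the damage volume.
; BI_PLayeRat actors take one NoIFrame hit on entering, re-armed when one leaves.
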(event OnComponentBeginOverlap(checkforcolluon)
  (params (OverlappedComponent :type Primitive%20Component%20Object%20Reference) (OtherActor :type Actor%20Object%20Reference) (OtherComp :type Primitive%20Component%20Object%20Reference) (OtherBodyIndex :type Integer) (bFromSweep :type Boolean) (SweepResult :type Hit%20Result%20Structure%20%28by%20ref%29))
  (if (Utilities|DoesObjectImplementInterface OtherActor "/Game/Rod3nt/Programming/BPI+Data/BI_Physics.BI_Physics_C")
    (Physics|SetSimulatePhysics (Variables|Default|GetStaticMesh) true)
    (bind _returnvalue (Utilities|Time|SetTimerbyEvent (delegate Custom|Check%20if%20Moving?) 0.1 true))
    (Variables|Default|SetTimer _returnvalue)))

(event OnComponentEndOverlap(dmg)
  (params (OverlappedComponent :type Primitive%20Component%20Object%20Reference) (OtherActor :type Actor%20Object%20Reference) (OtherComp :type Primitive%20Component%20Object%20Reference) (OtherBodyIndex :type Integer))
  (if (Utilities|DoesObjectImplementInterface OtherActor "/Game/Rod3nt/Programming/BPI+Data/BI_PlayeRat.BI_PLayeRat_C")
    (Utilities|FlowControl|DoOnce false) ; enters at Reset
  ))

(event OnComponentBeginOverlap(dmg)
  (params (OverlappedComponent :type Primitive%20Component%20Object%20Reference) (OtherActor :type Actor%20Object%20Reference) (OtherComp :type Primitive%20Component%20Object%20Reference) (OtherBodyIndex :type Integer) (bFromSweep :type Boolean) (SweepResult :type Hit%20Result%20Structure%20%28by%20ref%29))
  (if (Utilities|DoesObjectImplementInterface OtherActor "/Game/Rod3nt/Programming/BPI+Data/BI_PlayeRat.BI_PLayeRat_C")
    (Utilities|FlowControl|DoOnce false
      (:Completed
        (Game|Damage|ApplyDamage OtherActor 2.0 0 0 "/Game/Rod3nt/Programming/BPI+Data/NoIFrame.NoIFrame_C")))))

(event Custom|Check%20if%20Moving?
  (bind _grounded_ (Utilities|DetectSpeed (Variables|Default|GetStaticMesh))
    (:Out
      (if _grounded_
        (Components|Activation|SetActive (Variables|Default|GetNS_Poison) true false)
        (Collision|SetCollisionEnabled (Variables|Default|Getdmg) "QueryOnly")
        (Utilities|Time|ClearandInvalidateTimerbyHandle (Variables|Default|GetTimer))
        (Utilities|FlowControl|DoOnce false
          (:Completed
            ;[0.15 0.15 0.15 0.5] New Poison cloud vfx works now - J
            (Niagara|SpawnSystemAttached "/Game/Rod3nt/VFX/Poison/NS_PoisonExplosion.NS_PoisonExplosion" (Variables|Default|GetStaticMesh) "None" "0, 0, 0" "0, 0, 0" "KeepRelativeOffset" false)
            (Niagara|SpawnSystematLocation "/Game/Rod3nt/VFX/Poison/NS_PoisonText.NS_PoisonText" (Transformation|GetActorLocation))))))))

(event Collision|EventActorBeginOverlap
  (params (OtherActor :type Actor%20Object%20Reference)))

(event EventTick
  (params (DeltaSeconds :type Float%20%28single-precision%29)))

(event EventBeginPlay
  (Collision|SetCollisionEnabled (Variables|Default|Getdmg) "NoCollision"))

(fn ConstructionScript)