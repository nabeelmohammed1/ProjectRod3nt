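; BP_MapBounds is a tool actor that shows the 2D world bounds of the area covered by its Box collision component.
; BeginPlay derives X/Y min and max from the box's world location and scaled extent, passing them to the otherwise empty PrintBounds event.
; Tick reads that event's parameters and prints both corners on screen every frame.
; Overlap events are empty, and leftover controller-destroy nodes never run.
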(event OnComponentEndOverlap(Box)
  (params (OverlappedComponent :type Primitive%20Component%20Object%20Reference) (OtherActor :type Actor%20Object%20Reference) (OtherComp :type Primitive%20Component%20Object%20Reference) (OtherBodyIndex :type Integer)))

(event OnComponentBeginOverlap(Box)
  (params (OverlappedComponent :type Primitive%20Component%20Object%20Reference) (OtherActor :type Actor%20Object%20Reference) (OtherComp :type Primitive%20Component%20Object%20Reference) (OtherBodyIndex :type Integer) (bFromSweep :type Boolean) (SweepResult :type Hit%20Result%20Structure%20%28by%20ref%29)))

(event Custom|Print%20bounds
  (params (Box%20Vector :type Vector) (World%20LOC :type Vector) (World%20Min :type Vector%202D%20Structure) (World%20Max :type Vector%202D%20Structure)))

(event EventBeginPlay
  (bind _box (Variables|Default|GetBox))
  (bind _box_2 (Variables|Default|GetBox))
  (bind _returnvalue (Transformation|GetWorldLocation _box))
  (bind _returnvalue_2 (Components|Box|GetScaledBoxExtent _box_2))
  ;[0.15 0.15 0.15 0.5] Get's the Collision's values and prints out the Min/Max values
  (CallFunction|PrintBounds "0, 0, 0" "0, 0, 0" (Math|Vector2D|MakeVector2D (- (.x _returnvalue) (.x _returnvalue_2)) (- (.y _returnvalue) (.y _returnvalue_2))) (Math|Vector2D|MakeVector2D (+ (.x _returnvalue) (.x _returnvalue_2)) (+ (.y _returnvalue) (.y _returnvalue_2)))))

(event EventTick
  (params (DeltaSeconds :type Float%20%28single-precision%29))
  (Development|PrintString (Utilities|String|ToString(Vector2d) (stale Custom|Print%20bounds World%20Min)) true true "(R=1.000000,G=0.000000,B=0.025116,A=1.000000)" 0.1)
  (Development|PrintString (Utilities|String|ToString(Vector2d) (stale Custom|Print%20bounds World%20Max)) true true "(R=0.000000,G=0.660000,B=1.000000,A=1.000000)" 0.1))

(fn ConstructionScript)