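; BP_SmoothCamera is a trigger box that eases the player's spring arm length as they enter and leave it.
; On begin overlap it caches the arm length, then a timeline lerps it toward 5 units shorter.
; On end overlap a second timeline lerps from that cached value toward 5 units longer, rather than back to it.
; DoOnce gates block retriggering until each timeline finishes.
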(event OnComponentBeginOverlap(Box)
  (params (OverlappedComponent :type Primitive%20Component%20Object%20Reference) (OtherActor :type Actor%20Object%20Reference) (OtherComp :type Primitive%20Component%20Object%20Reference) (OtherBodyIndex :type Integer) (bFromSweep :type Boolean) (SweepResult :type Hit%20Result%20Structure%20%28by%20ref%29))
  (bind _returnvalue (Actor|GetComponentbyClass OtherActor "/Script/Engine.SpringArmComponent"))
  (if (== OtherActor (Game|Player|GetPlayerPawn 0))
    (Utilities|IsValid _returnvalue
      (:Is%20Valid
        (Variables|Default|SetCachedLenght (Variables|/Script/Engine.SpringArmComponent|GetTargetArmLength _returnvalue))
        (Utilities|FlowControl|DoOnce false :!label _label
          (:Completed
            (bind _spring_arm (Timeline|Timeline PlayFromStart)
              (:Update
                (Variables|/Script/Engine.SpringArmComponent|SetTargetArmLength _returnvalue (Math|Float|Lerp (Variables|Default|GetCachedLenght) (- (Variables|Default|GetCachedLenght) 5.0) _spring_arm))
                (Development|PrintString "start updating"))
              (:Finished
                (Development|PrintString "reset this mf")
                (goto _label Reset)))))))))

(event OnComponentEndOverlap(Box)
  (params (OverlappedComponent :type Primitive%20Component%20Object%20Reference) (OtherActor :type Actor%20Object%20Reference) (OtherComp :type Primitive%20Component%20Object%20Reference) (OtherBodyIndex :type Integer))
  (bind _returnvalue (Actor|GetComponentbyClass OtherActor "/Script/Engine.SpringArmComponent"))
  (bind _cachedlenght (Variables|Default|GetCachedLenght))
  (if (== OtherActor (Game|Player|GetPlayerPawn 0))
    (Utilities|IsValid _returnvalue
      (:Is%20Valid
        (Utilities|FlowControl|DoOnce false :!label _label
          (:Completed
            (bind _spring_arm (Timeline|Timeline_0 PlayFromStart)
              (:Update
                (Variables|/Script/Engine.SpringArmComponent|SetTargetArmLength _returnvalue (Math|Float|Lerp _cachedlenght (+ _cachedlenght 5.0) _spring_arm))
                (Development|PrintString "end reset"))
              (:Finished
                (Development|PrintString "we need thr reset")
                (goto _label Reset)))))))))

(event EventBeginPlay)

(fn ConstructionScript)