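; BP_ThrowRock is a thrown rock projectile that makes noise on impact and turns back into a pickup.
; SetImpulse launches its static mesh, and the first hit on anything but its instigator plays a sound and Niagara effect and reports a noise event.
; Timers set at BeginPlay drive the stop check and timeout.
; Coming to rest or exploding replaces it with a BP_PickupRock at its transform.
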(event Custom|IsStopped?
  (if (< (Math|Vector|VectorLength (Transformation|GetComponentVelocity (Variables|Default|GetStaticMesh))) 0.01)
    (Utilities|FlowControl|DoOnce false
      (:Completed
        (Game|SpawnActorfromClass "/Game/Rod3nt/Programming/PICKUPSandENVI-BPS/BP_PickupRock.BP_PickupRock_C" (Math|Transform|MakeTransform (Transformation|GetActorLocation) (Transformation|GetActorRotation) "1.000000,1.000000,1.000000") "Undefined" "MultiplyWithRoot" 0 0)
        (Actor|DestroyActor)))))

(event Custom|Explode
  (Utilities|Time|ClearandInvalidateTimerbyHandle (stale EventBeginPlay _returnvalue))
  (Game|SpawnActorfromClass "/Game/Rod3nt/Programming/PICKUPSandENVI-BPS/BP_PickupRock.BP_PickupRock_C" (Math|Transform|MakeTransform (Transformation|GetActorLocation) (Transformation|GetActorRotation) "1.000000,1.000000,1.000000") "Undefined" "MultiplyWithRoot" 0 0)
  (Actor|DestroyActor))

(event EventBeginPlay
  (bind _returnvalue (Utilities|Time|SetTimerbyEvent (EventDispatchers|CreateEvent :!event Custom|IsStopped?) 0.2 true))
  (Utilities|Time|SetTimerbyEvent (EventDispatchers|CreateEvent :!event Custom|Explode) 3.0))

(event EventSetImpulse
  (params (X :type Float%20%28double-precision%29) (Y :type Float%20%28double-precision%29) (Z :type Float%20%28double-precision%29))
  (Physics|AddImpulse (Variables|Default|GetStaticMesh) (Math|Vector|MakeVector X Y Z) "None" true))

(event Collision|EventHit
  (params (MyComp :type Primitive%20Component%20Object%20Reference) (Other :type Actor%20Object%20Reference) (OtherComp :type Primitive%20Component%20Object%20Reference) (bSelfMoved :type Boolean) (HitLocation :type Vector :default "0, 0, 0") (HitNormal :type Vector :default "0, 0, 0") (NormalImpulse :type Vector :default "0, 0, 0") (Hit :type Hit%20Result%20Structure%20%28by%20ref%29))
  (if (not (== (Game|GetInstigator) Other))
    (Utilities|FlowControl|DoOnce false
      (:Completed
        (Audio|PlaySoundatLocation "/Game/Rod3nt/sounds/bullet-shells-hitting-ground_Cue.bullet-shells-hitting-ground_Cue" HitLocation "0, 0, 0" 1.0 1.0 0.0 0 0 0 0)
        (Niagara|SpawnSystematLocation "/Game/Rod3nt/VFX/Rock/NS_Rock.NS_Rock" (+ (Transformation|GetActorLocation) "0.000000,0.000000,100.000000"))
        (Class|AISenseHearing|ReportNoiseEvent HitLocation 1.0 self 0.0 "None")))))

(fn ConstructionScript)