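; BP_RPG is an RPG projectile or blast actor that damages and knocks back what it touches, and destroys itself after BulletHalflife.
; When its Sphere overlaps a BI_Damage actor, it launches that actor away along the center-to-center direction, scaled by Knockback horizontally and a fixed factor vertically.
; It then sends fixed damage through both ApplyDamage and an interface message.
; Overlaps do not destroy it; only the timer does.
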(event OnComponentBeginOverlap(Sphere)
  (params (OverlappedComponent :type Primitive%20Component%20Object%20Reference) (OtherActor :type Actor%20Object%20Reference) (OtherComp :type Primitive%20Component%20Object%20Reference) (OtherBodyIndex :type Integer) (bFromSweep :type Boolean) (SweepResult :type Hit%20Result%20Structure%20%28by%20ref%29))
  (bind _returnvalue (Transformation|GetActorLocation OtherActor))
  (bind _returnvalue_2 (Transformation|GetActorLocation))
  (bind _knockback (Variables|Default|Getknockback))
  (bind _returnvalue_3 (- _returnvalue _returnvalue_2))
  (bind _returnvalue_4 (Math|Vector|Normalize _returnvalue_3))
  (bind _returnvalue_5 (* _returnvalue_4 _knockback))
  (if (Utilities|DoesObjectImplementInterface OtherActor "/Game/Rod3nt/Programming/BPI+Data/BI_Damage.BI_Damage_C")
    (Class|BIDamage|LaunchPlayer(Message) OtherActor (Math|Vector|MakeVector (.x _returnvalue_5) (.y _returnvalue_5) (.z (* _returnvalue_4 5e+03))))
    (Game|Damage|ApplyDamage OtherActor 1e+01 0 0 (Variables|Default|GetDamage%20Type%20Class))
    (Class|BIDamage|ReceiveDmg(Message) OtherActor 1e+01)))

(event Custom|DestroyBullet
  (Actor|DestroyActor))

(event EventBeginPlay
  (Utilities|Time|SetTimerbyEvent (delegate Custom|DestroyBullet) (Variables|Default|GetBulletHalflife)))

(event EventTick
  (params (DeltaSeconds :type Float%20%28single-precision%29)))

(fn ConstructionScript)