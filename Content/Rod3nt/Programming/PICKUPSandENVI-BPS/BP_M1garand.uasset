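; BP_M1garand is an M1 Garand physics prop that fires once knocked and come to rest.
; Overlap by a BI_Physics actor enables heavy physics and starts a looping timer that fires when velocity is near zero, then clears itself.
; Firing reports noise, plays muzzle effects and launches a BP_RifleBullet.
; SendFlying applies an impulse; the player's first overlap shows a UI message and flags every instance to suppress repeats.
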(event OnComponentBeginOverlap(Box)
  (params (OverlappedComponent :type Primitive%20Component%20Object%20Reference) (OtherActor :type Actor%20Object%20Reference) (OtherComp :type Primitive%20Component%20Object%20Reference) (OtherBodyIndex :type Integer) (bFromSweep :type Boolean) (SweepResult :type Hit%20Result%20Structure%20%28by%20ref%29))
  (bind _m1garand (Variables|Default|GetM1Garand))
  (if (Utilities|DoesObjectImplementInterface OtherActor "/Game/Rod3nt/Programming/BPI+Data/BI_Physics.BI_Physics_C")
    (Physics|SetSimulatePhysics _m1garand true)
    (Class|PrimitiveComponent|SetMassOverrideinKg _m1garand "None" 6e+02 true)
    (bind _returnvalue (Utilities|Time|SetTimerbyEvent (delegate Custom|Check%20if%20Moving?) 0.2 true))
    (Variables|Default|SetMovingTimer _returnvalue)
    (if (== OtherActor (Game|Player|GetPlayerPawn 0))
      (if (not (Variables|Default|GetGunShotted))
        (Utilities|FlowControl|DoOnce false
          (:Completed
            (Class|BIPLayeRat|UIforCapy(Message) OtherActor "NewEnumerator3")
            (bind _outactors (Actor|GetAllActorsOfClass "BP_M1garand_C"))
            (for _array_element _outactors
              (Variables|BP_M1garand_C|SetGunShotted _array_element true)))))
      (else
        (Development|PrintString "not")))))

(event Custom|Check%20if%20Moving?
  (bind _grounded_ (Utilities|DetectSpeed (Variables|Default|GetM1Garand))
    (:Out
      (if _grounded_
        (CallFunction|FireGun)
        (Utilities|Time|ClearandInvalidateTimerbyHandle (Variables|Default|GetMovingTimer))))))

(event Custom|FireGun
  (bind _bulletspawn (Variables|Default|GetBulletSpawn))
  (bind _arrow (Variables|Default|GetArrow))
  (bind _returnvalue (Transformation|GetWorldTransform _bulletspawn))
  (bind _returnvalue_2 (Transformation|GetWorldLocation _arrow))
  (Class|AISenseHearing|ReportNoiseEvent _returnvalue_2 1.0 self 0.0 "0")
  (Niagara|SpawnSystematLocation "/Game/Rod3nt/VFX/MuzzleFlash/NS_MuzzleFlash.NS_MuzzleFlash" _returnvalue_2)
  (Audio|PlaySoundatLocation "/Game/Rod3nt/sounds/pistol-shot-233473_Cue.pistol-shot-233473_Cue" (Transformation|GetWorldLocation (Variables|Default|GetArrow)) "0, 0, 0" 0.5 1.0 0.0 "/Game/Rod3nt/sounds/gunshot1.gunshot1" 0 0 0)
  (bind _returnvalue_3 (Game|SpawnActorfromClass "/Game/Rod3nt/Programming/PICKUPSandENVI-BPS/BP_RifleBullet.BP_RifleBullet_C" (Math|Transform|MakeTransform (.location _returnvalue) (.rotation _returnvalue) "1.000000,1.000000,1.000000") "Undefined" "MultiplyWithRoot" 0 0))
  (Physics|AddImpulse (Variables|/Game/Rod3nt/Programming/PICKUPSandENVI-BPS/BP_RifleBullet.BP_RifleBullet_C|GetBulletBase _returnvalue_3) (* (Math|Vector|GetForwardVector (Variables|Default|GetBulletSpawn)) (Variables|Default|GetBulletForce)) "None" true))

(event Collision|EventActorBeginOverlap
  (params (OtherActor :type Actor%20Object%20Reference)))

(event EventTick
  (params (DeltaSeconds :type Float%20%28single-precision%29)))

(event EventSendFlying
  (params (Launch%20Vel :type Float%20%28double-precision%29))
  (bind _m1garand (Variables|Default|GetM1Garand))
  (Physics|SetSimulatePhysics _m1garand true)
  (Class|PrimitiveComponent|SetMassOverrideinKg _m1garand "None" 6e+02 true)
  (Physics|AddImpulse (Variables|Default|GetM1Garand) (Math|Conversions|ToVector(Float) Launch%20Vel) "None" false))

(event EventTurnon)

(event EventTurnOff)

(fn ConstructionScript)