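; BP_RifleBullet is a rifle projectile actor that damages what it hits and destroys itself after a timer set by BulletHalflife.
; Each tick it rotates the bullet mesh to face the velocity of BulletBase.
; When BulletArea overlaps an actor implementing BI_Damage, it applies fixed damage through the engine's ApplyDamage and destroys itself.
; Overlaps with actors lacking that interface are ignored, so the bullet persists.
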(event OnComponentBeginOverlap(BulletArea)
  (params (OverlappedComponent :type Primitive%20Component%20Object%20Reference) (OtherActor :type Actor%20Object%20Reference) (OtherComp :type Primitive%20Component%20Object%20Reference) (OtherBodyIndex :type Integer) (bFromSweep :type Boolean) (SweepResult :type Hit%20Result%20Structure%20%28by%20ref%29))
  (if (Utilities|DoesObjectImplementInterface OtherActor "/Game/Rod3nt/Programming/BPI+Data/BI_Damage.BI_Damage_C")
    (Game|Damage|ApplyDamage OtherActor 3.0 0 0)
    (Actor|DestroyActor)))

(event Custom|DestroyBullet
  (Actor|DestroyActor))

(event EventBeginPlay
  (Utilities|Time|SetTimerbyEvent (delegate Custom|DestroyBullet) (Variables|Default|GetBulletHalflife)))

(event EventTick
  (params (DeltaSeconds :type Float%20%28single-precision%29))
  (Transformation|SetWorldRotation (Variables|Default|Getsm_Bullet2) (Math|Rotator|MakeRotfromX (Transformation|GetComponentVelocity (Variables|Default|GetBulletBase))) false false))

(fn ConstructionScript)