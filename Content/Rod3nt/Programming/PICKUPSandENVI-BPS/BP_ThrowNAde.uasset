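; Thrown grenade actor that takes a launch impulse and explodes on a short fuse, or sooner once it stops moving.
; A looping timer polls the mesh's velocity for rest, alongside the fuse timer.
; Its first hit on anything but the instigator reports a noise event.
; Explosion spawns Niagara and sound, launches and damages overlapping BI_Physics actors within its sphere, then destroys itself.
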(event Custom|CheckforStopping
  (bind _grounded_ (Utilities|DetectSpeed (Variables|Default|GetStaticMesh))
    (:Out
      (if _grounded_
        (CallFunction|ExplodeNade)
        (Utilities|Time|ClearandInvalidateTimerbyHandle (stale EventBeginPlay _returnvalue))
        (Utilities|Time|ClearandInvalidateTimerbyHandle (stale EventBeginPlay _returnvalue_2))))))

(event Custom|ExplodeNade
  (bind _returnvalue (Transformation|GetActorLocation))
  (Niagara|SpawnSystematLocation "/Game/Rod3nt/VFX/Explosion/NS_GrenadeExplosion.NS_GrenadeExplosion" _returnvalue)
  (CallFunction|Explodeothers)
  (Audio|PlaySoundatLocation "/Game/Rod3nt/sounds/GrenadeBoom_Cue.GrenadeBoom_Cue" _returnvalue "0, 0, 0" 1.0 1.0 0.0 0 0 0 0))

(event Custom|Explodeothers
  (for _array_element (Collision|GetOverlappingActors (Variables|Default|GetSphere) 0 :!class /Script/Engine.PrimitiveComponent)
    (if (Utilities|DoesObjectImplementInterface _array_element "/Game/Rod3nt/Programming/BPI+Data/BI_Physics.BI_Physics_C")
      (Class|BIPhysics|SendFlying(Message) _array_element 8e+03)
      (Game|Damage|ApplyDamage _array_element 5.0 0 0 "/Game/Rod3nt/Programming/BPI+Data/NoIFrame.NoIFrame_C")))
  (Actor|DestroyActor))

(event Custom|Explode
  (CallFunction|ExplodeNade)
  (Utilities|Time|ClearandInvalidateTimerbyHandle (stale EventBeginPlay _returnvalue))
  (Utilities|Time|ClearandInvalidateTimerbyHandle (stale EventBeginPlay _returnvalue_2)))

(event EventBeginPlay
  (bind _returnvalue (Utilities|Time|SetTimerbyEvent (delegate Custom|CheckforStopping) 0.4 true))
  (bind _returnvalue_2 (Utilities|Time|SetTimerbyEvent (delegate Custom|Explode) 1.5)))

(event Collision|EventHit
  (params (MyComp :type Primitive%20Component%20Object%20Reference) (Other :type Actor%20Object%20Reference) (OtherComp :type Primitive%20Component%20Object%20Reference) (bSelfMoved :type Boolean) (HitLocation :type Vector :default "0, 0, 0") (HitNormal :type Vector :default "0, 0, 0") (NormalImpulse :type Vector :default "0, 0, 0") (Hit :type Hit%20Result%20Structure%20%28by%20ref%29))
  (if (not (== (Game|GetInstigator) Other))
    (Utilities|FlowControl|DoOnce false
      (:Completed
        (Class|AISenseHearing|ReportNoiseEvent HitLocation 1.0 self 0.0 "None")))))

(event EventSetImpulse
  (params (X :type Float%20%28double-precision%29) (Y :type Float%20%28double-precision%29) (Z :type Float%20%28double-precision%29))
  (Physics|AddImpulse (Variables|Default|GetStaticMesh) (Math|Vector|MakeVector X Y Z) "None" true))

(fn ConstructionScript)