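; BP_gunPPSH is a physics prop gun that fires a burst on its own after being knocked loose.
; Overlap by a BI_Physics actor enables heavy physics and starts a timer that waits until the gun is nearly still.
; A second looping timer then fires a short burst of impulse-driven BP_RifleBullets with flash, sound and noise events.
; SendFlying launches the gun by impulse but does not start the rest check.
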(event OnComponentBeginOverlap(Box)
  (params (OverlappedComponent :type Primitive%20Component%20Object%20Reference) (OtherActor :type Actor%20Object%20Reference) (OtherComp :type Primitive%20Component%20Object%20Reference) (OtherBodyIndex :type Integer) (bFromSweep :type Boolean) (SweepResult :type Hit%20Result%20Structure%20%28by%20ref%29))
  (bind _ppsh (Variables|Default|GetPPSH))
  (if (Utilities|DoesObjectImplementInterface OtherActor "/Game/Rod3nt/Programming/BPI+Data/BI_Physics.BI_Physics_C")
    (Physics|SetSimulatePhysics _ppsh true)
    (Class|PrimitiveComponent|SetMassOverrideinKg _ppsh "None" 6e+02 true)
    (bind _returnvalue (Utilities|Time|SetTimerbyEvent (delegate Custom|Check%20if%20Moving?) 0.2 true))
    (Variables|Default|SetMovingTimer _returnvalue)))

(event Custom|Check%20if%20Moving?
  (bind _grounded_ (Utilities|DetectSpeed (Variables|Default|GetPPSH))
    (:Out
      (if _grounded_
        (CallFunction|FireGun)
        (Utilities|Time|ClearandInvalidateTimerbyHandle (Variables|Default|GetMovingTimer))))))

(event Custom|FireGun
  (bind _returnvalue (Utilities|Time|SetTimerbyEvent (delegate Custom|fire%20lofic) 0.2 true)))

(event Custom|fire%20lofic
  (bind _bulletspawn (Variables|Default|GetBulletSpawn))
  (bind _returnvalue (Transformation|GetWorldTransform _bulletspawn))
  (Math|Integer|IncrementInt (Variables|Default|GettimesShot)
    (:%20%20
      (Niagara|SpawnSystematLocation "/Game/Rod3nt/VFX/MuzzleFlash/NS_MuzzleFlash.NS_MuzzleFlash" (Transformation|GetWorldLocation (Variables|Default|GetArrow)))
      (Audio|PlaySoundatLocation "/Game/Rod3nt/sounds/machine-gun-5_Cue.machine-gun-5_Cue" (Transformation|GetWorldLocation (Variables|Default|GetArrow)) "0, 0, 0" 0.5 1.0 0.0 "/Game/Rod3nt/sounds/gunshot1.gunshot1" 0 0 0)
      (Class|AISenseHearing|ReportNoiseEvent (.location _returnvalue) 1.0 self 0.0 "None")
      (bind _returnvalue_2 (Game|SpawnActorfromClass "/Game/Rod3nt/Programming/PICKUPSandENVI-BPS/BP_RifleBullet.BP_RifleBullet_C" (Math|Transform|MakeTransform (.location _returnvalue) (.rotation _returnvalue) "1.000000,1.000000,1.000000") "Undefined" "MultiplyWithRoot" 0 0))
      (Physics|AddImpulse (Variables|/Game/Rod3nt/Programming/PICKUPSandENVI-BPS/BP_RifleBullet.BP_RifleBullet_C|GetBulletBase _returnvalue_2) (* (Math|Vector|GetForwardVector (Variables|Default|GetBulletSpawn)) (Variables|Default|GetBulletForce)) "None" true)
      (if (>= (Variables|Default|GettimesShot) 6)
        (Utilities|Time|ClearandInvalidateTimerbyHandle (stale Custom|FireGun _returnvalue))
        (Variables|Default|SettimesShot 0)))))

(event EventBeginPlay)

(event Collision|EventActorBeginOverlap
  (params (OtherActor :type Actor%20Object%20Reference)))

(event Collision|EventHit
  (params (MyComp :type Primitive%20Component%20Object%20Reference) (Other :type Actor%20Object%20Reference) (OtherComp :type Primitive%20Component%20Object%20Reference) (bSelfMoved :type Boolean) (HitLocation :type Vector :default "0, 0, 0") (HitNormal :type Vector :default "0, 0, 0") (NormalImpulse :type Vector :default "0, 0, 0") (Hit :type Hit%20Result%20Structure%20%28by%20ref%29)))

(event EventSendFlying
  (params (Launch%20Vel :type Float%20%28double-precision%29))
  (bind _ppsh (Variables|Default|GetPPSH))
  (Physics|SetSimulatePhysics _ppsh true)
  (Class|PrimitiveComponent|SetMassOverrideinKg _ppsh "None" 6e+02 true)
  (Physics|AddImpulse (Variables|Default|GetPPSH) (Math|Conversions|ToVector(Float) Launch%20Vel) "None" false))

(event EventTurnon)

(event EventTurnOff)

(fn ConstructionScript)