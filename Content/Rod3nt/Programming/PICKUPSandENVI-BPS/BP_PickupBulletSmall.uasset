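; Small bullet pickup that the rat player can carry on its back, one pickup at a time.
; A sphere overlap shows an interact widget; interacting inside it sends mesh, icon, throw class, move speed and scale through PickuponBackMessage, then destroys the actor.
; Separate events toggle custom depth rendering on the mesh and a billboard icon, which overlap re-shows while enabled.
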(event OnComponentBeginOverlap(Sphere)
  (params (OverlappedComponent :type Primitive%20Component%20Object%20Reference) (OtherActor :type Actor%20Object%20Reference) (OtherComp :type Primitive%20Component%20Object%20Reference) (OtherBodyIndex :type Integer) (bFromSweep :type Boolean) (SweepResult :type Hit%20Result%20Structure%20%28by%20ref%29))
  (if (Utilities|DoesObjectImplementInterface OtherActor "/Game/Rod3nt/Programming/BPI+Data/BI_PlayeRat.BI_PLayeRat_C")
    (Variables|/Script/UMG.Widget|SetVisibility (stale EventBeginPlay _returnvalue) "Visible")
    (if (Variables|Default|Getbillboard%20on)
      (Development|SetHiddeninGame (Variables|Default|GetBillboard) false false))))

(event OnComponentEndOverlap(Sphere)
  (params (OverlappedComponent :type Primitive%20Component%20Object%20Reference) (OtherActor :type Actor%20Object%20Reference) (OtherComp :type Primitive%20Component%20Object%20Reference) (OtherBodyIndex :type Integer))
  (if (Utilities|DoesObjectImplementInterface OtherActor "/Game/Rod3nt/Programming/BPI+Data/BI_PlayeRat.BI_PLayeRat_C")
    (Variables|/Script/UMG.Widget|SetVisibility (stale EventBeginPlay _returnvalue) "Hidden")))

(event Input|EnhancedActionEvents|EnhancedInputActionIA_Interact1
  (params (ActionValue :type Vector%202D%20Structure) (ElapsedSeconds :type Float%20%28double-precision%29) (TriggeredSeconds :type Float%20%28double-precision%29) (InputAction :type Input%20Action%20Object%20Reference :default "/Game/Input/Actions/IA_Interact1.IA_Interact1"))
  (bind _returnvalue (Game|GetPlayerCharacter 0))
  (:Completed
    (if (Collision|IsOverlappingActor (Variables|Default|GetSphere) (Game|GetPlayerCharacter 0) :!class /Script/Engine.PrimitiveComponent)
      (bind _pickup (Class|BIPLayeRat|HasPickup?(Message) _returnvalue))
      (if (not _pickup)
        (Class|BIPLayeRat|PickuponBack(Message) _returnvalue (Utilities|Struct|MakeS_PickupData (Variables|/Script/Engine.StaticMeshComponent|GetStaticMesh (Variables|Default|GetStaticMesh)) "/Game/Rod3nt/UIArt/FinalUIElements/NewRodentHud/Bulletr.Bulletr" (Variables|Default|GetThrowClassRef) 5.0 "5.000000,5.000000,5.000000"))
        (Actor|DestroyActor)))))

(event EventBeginPlay
  (Input|EnableInput (Game|GetPlayerController 0))
  (bind _returnvalue (UserInterface|CreateWidget "/Game/Rod3nt/Programming/UI/WBP_Interact.WBP_Interact_C"))
  (UserInterface|Viewport|AddtoViewport _returnvalue 0)
  (Variables|/Script/UMG.Widget|SetVisibility _returnvalue "Hidden"))

(event EventMakeiconappear
  (Variables|Default|Setbillboard%20on true)
  (Development|SetHiddeninGame (Variables|Default|GetBillboard) false false))

(event EventMakeiconDisappear
  (Variables|Default|Setbillboard%20on false)
  (Development|SetHiddeninGame (Variables|Default|GetBillboard) true false))

(event EventTurnon
  (Rendering|SetRenderCustomDepth (Variables|Default|GetStaticMesh) true))

(event EventTurnOff
  (Rendering|SetRenderCustomDepth (Variables|Default|GetStaticMesh) false))

(fn ConstructionScript)