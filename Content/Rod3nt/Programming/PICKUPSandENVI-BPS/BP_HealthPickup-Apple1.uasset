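; Apple health pickup that restores player health when interacted with inside its sphere, then plays a sound and destroys itself.
; Sphere overlaps with BI_PLayeRat actors toggle an interact widget, created at BeginPlay, and a billboard icon.
; The actor enables its own input and checks overlap when IA_Interact1 completes, sending HealthBoost through GetBackHealthMessage.
; Separate events control the icon and custom-depth rendering on the mesh, and PlayerDist offers a range check.
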(event OnComponentBeginOverlap(Sphere)
  (params (OverlappedComponent :type Primitive%20Component%20Object%20Reference) (OtherActor :type Actor%20Object%20Reference) (OtherComp :type Primitive%20Component%20Object%20Reference) (OtherBodyIndex :type Integer) (bFromSweep :type Boolean) (SweepResult :type Hit%20Result%20Structure%20%28by%20ref%29))
  (if (Utilities|DoesObjectImplementInterface OtherActor "/Game/Rod3nt/Programming/BPI+Data/BI_PlayeRat.BI_PLayeRat_C")
    (Variables|/Script/UMG.Widget|SetVisibility (Variables|Default|GetWidget) "Visible")
    (if (not (Variables|Default|Getbillboard%20on))
      (Development|SetHiddeninGame (Variables|Default|GetBillboard) false false))))

(event OnComponentEndOverlap(Sphere)
  (params (OverlappedComponent :type Primitive%20Component%20Object%20Reference) (OtherActor :type Actor%20Object%20Reference) (OtherComp :type Primitive%20Component%20Object%20Reference) (OtherBodyIndex :type Integer))
  (if (Utilities|DoesObjectImplementInterface OtherActor "/Game/Rod3nt/Programming/BPI+Data/BI_PlayeRat.BI_PLayeRat_C")
    (Variables|/Script/UMG.Widget|SetVisibility (Variables|Default|GetWidget) "Hidden")
    (Development|SetHiddeninGame (Variables|Default|GetBillboard) true false)))

(event Input|EnhancedActionEvents|EnhancedInputActionIA_Interact1
  (params (ActionValue :type Vector%202D%20Structure) (ElapsedSeconds :type Float%20%28double-precision%29) (TriggeredSeconds :type Float%20%28double-precision%29) (InputAction :type Input%20Action%20Object%20Reference :default "/Game/Input/Actions/IA_Interact1.IA_Interact1"))
  (bind _returnvalue (Game|GetPlayerCharacter 0))
  (:Completed
    (if (Collision|IsOverlappingActor (Variables|Default|GetSphere) _returnvalue :!class /Script/Engine.PrimitiveComponent)
      (Class|BIPLayeRat|GetBackHealth(Message) _returnvalue (Variables|Default|GetHealth%20Boost))
      (Audio|PlaySoundatLocation 0 (Transformation|GetWorldLocation (Variables|Default|GetStaticMesh)) "0, 0, 0" 1.0 1.0 0.0 0 0 0 0)
      (Actor|DestroyActor))))

(event EventBeginPlay
  (Input|EnableInput (Game|GetPlayerController 0))
  (bind _returnvalue (UserInterface|CreateWidget "/Game/Rod3nt/Programming/UI/WBP_Interact.WBP_Interact_C"))
  (Variables|Default|SetWidget _returnvalue)
  (UserInterface|Viewport|AddtoViewport _returnvalue 0)
  (Variables|/Script/UMG.Widget|SetVisibility _returnvalue "Hidden"))

(event EventMakeiconappear
  (Variables|Default|Setbillboard%20on true)
  (Development|SetHiddeninGame (Variables|Default|GetBillboard) false false))

(event EventMakeiconDisappear
  (Variables|Default|Setbillboard%20on false)
  (Development|SetHiddeninGame (Variables|Default|GetBillboard) true false))

(event EventTurnon
  (Rendering|SetRenderCustomDepth (Variables|Default|GetStaticMesh) true))

(event EventTurnOff
  (Rendering|SetRenderCustomDepth (Variables|Default|GetStaticMesh) false))

(fn ConstructionScript)

(fn PlayerDist
  (return (<= (Math|Vector|Distance(Vector) (Transformation|GetActorLocation) (Transformation|GetActorLocation (Game|Player|GetPlayerPawn 0))) (Variables|Default|GetDistance%20from%20Player))))