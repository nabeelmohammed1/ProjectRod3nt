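; BP_BulletBig is a physics-driven big bullet that acts as a noise source and turns back into a pickup once it comes to rest.
; SetImpulse launches the mesh, and its first non-instigator hit plays a shell sound, reports an AI noise event and spawns a clink effect.
; A velocity check, likely polled by the looping timer, replaces the stopped actor with BP_PickupBulletBig and plays a sound.
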(event Custom|IsStopped?
  (if (< (Math|Vector|VectorLength (Transformation|GetComponentVelocity (Variables|Default|GetStaticMesh))) 0.01)
    (Utilities|FlowControl|DoOnce false
      (:Completed
        (Game|SpawnActorfromClass "/Game/Rod3nt/Programming/PICKUPSandENVI-BPS/BP_PickupBulletBig.BP_PickupBulletBig_C" (Math|Transform|MakeTransform (Transformation|GetActorLocation) (Transformation|GetActorRotation) (Transformation|GetWorldScale (Variables|Default|GetStaticMesh))) "Undefined" "MultiplyWithRoot" 0 0)
        (Audio|SpawnSoundatLocation "/Game/Rod3nt/sounds/Grenade-pin_Cue.Grenade-pin_Cue" (Transformation|GetWorldLocation (Variables|Default|GetStaticMesh)) "0, 0, 0" 1.0 1.0 0.0 0 0)
        (Actor|DestroyActor)))))

(event EventBeginPlay
  (Utilities|Time|SetTimerbyEvent (EventDispatchers|CreateEvent :!event Custom|IsStopped?) 0.2 true))

(event Collision|EventActorBeginOverlap
  (params (OtherActor :type Actor%20Object%20Reference)))

(event Collision|EventHit
  (params (MyComp :type Primitive%20Component%20Object%20Reference) (Other :type Actor%20Object%20Reference) (OtherComp :type Primitive%20Component%20Object%20Reference) (bSelfMoved :type Boolean) (HitLocation :type Vector :default "0, 0, 0") (HitNormal :type Vector :default "0, 0, 0") (NormalImpulse :type Vector :default "0, 0, 0") (Hit :type Hit%20Result%20Structure%20%28by%20ref%29))
  (if (== (Game|GetInstigator) Other)
    (Development|PrintString "yes")
    (else
      (Utilities|FlowControl|DoOnce false
        (:Completed
          (Audio|PlaySoundatLocation "/Game/Rod3nt/sounds/bullet-shells-hitting-ground_Cue.bullet-shells-hitting-ground_Cue" HitLocation "0, 0, 0" 1.0 1.0 0.0 0 0 0 0)
          (Class|AISenseHearing|ReportNoiseEvent HitLocation 1.0 self 0.0 "None")
          (Niagara|SpawnSystematLocation "/Game/Rod3nt/VFX/Clink/NS_Clink.NS_Clink" (+ (Transformation|GetActorLocation) "0.000000,0.000000,100.000000")))))))

(event EventSetImpulse
  (params (X :type Float%20%28double-precision%29) (Y :type Float%20%28double-precision%29) (Z :type Float%20%28double-precision%29))
  (Physics|AddImpulse (Variables|Default|GetStaticMesh) (Math|Vector|MakeVector X Y Z) "None" true))

(fn ConstructionScript)