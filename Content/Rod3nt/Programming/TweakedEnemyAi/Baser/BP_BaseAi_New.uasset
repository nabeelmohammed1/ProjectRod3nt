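; BP_BaseAi_New is a base enemy AI character that can shoot the player and be stunned.
; A capsule overlap with an actor tagged "Stunnable" sets its blackboard stunned flag and attaches a stun Niagara effect above the mesh.
; The attack plays a shoot montage, directly damages the player pawn without any hit check, and returns the montage length plus a delay.
; A getter exposes its Path variable.
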(event OnComponentBeginOverlap(Capsule)
  (params (OverlappedComponent :type Primitive%20Component%20Object%20Reference) (OtherActor :type Actor%20Object%20Reference) (OtherComp :type Primitive%20Component%20Object%20Reference) (OtherBodyIndex :type Integer) (bFromSweep :type Boolean) (SweepResult :type Hit%20Result%20Structure%20%28by%20ref%29))
  (if (Actor|ActorHasTag OtherActor "Stunnable")
    (AI|Components|Blackboard|SetValueasBool (AI|GetBlackboard (Pawn|GetController)) (Utilities|Name|MakeLiteralName "Stunned?") true)
    (Niagara|SpawnSystemAttached "/Game/Rod3nt/VFX/Stunned/NS_Stunned.NS_Stunned" (Variables|Character|GetMesh) "None" "0.000000,0.000000,200.000000" "0, 0, 0" "KeepRelativeOffset" true)))

(fn ConstructionScript)

(fn AttackthePlayer
  (bind _returnvalue (Animation|PlayAnimMontage "/Game/Rod3nt/Soldiers/humantest/Shootingguy/AM_Shoot.AM_Shoot" 1.0 "None"))
  (Game|Damage|ApplyDamage (Game|Player|GetPlayerPawn 0) 5.0 0 0)
  (return (+ _returnvalue 2.0)))

(fn GetThepath
  (return (Variables|Default|GetPath)))