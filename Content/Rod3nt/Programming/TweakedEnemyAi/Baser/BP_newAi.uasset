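; Enemy AI character with swappable face materials that can kick, damage the player, be launched, get stunned or die.
; Taser damage or overlap with Stunnable actors sets the blackboard stun flag and plays stun effects; other damage kills.
; Death runs once, ragdolling the mesh with a dead face and effect, then destroys the actor after a delay.
; Events toggle custom-depth rendering and movement ticking, and a getter exposes its paths.
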(event OnComponentBeginOverlap(Capsule)
  (params (OverlappedComponent :type Primitive%20Component%20Object%20Reference) (OtherActor :type Actor%20Object%20Reference) (OtherComp :type Primitive%20Component%20Object%20Reference) (OtherBodyIndex :type Integer) (bFromSweep :type Boolean) (SweepResult :type Hit%20Result%20Structure%20%28by%20ref%29))
  (if (Actor|ActorHasTag OtherActor "Stunnable")
    (AI|Components|Blackboard|SetValueasBool (AI|GetBlackboard (Pawn|GetController)) (Utilities|Name|MakeLiteralName "Stunned?") true)
    (Niagara|SpawnSystemAttached "/Game/Rod3nt/VFX/Stunned/NS_Stunned.NS_Stunned" (Variables|Character|GetMesh) "None" "0.000000,0.000000,200.000000" "0, 0, 0" "KeepRelativeOffset" true)
    (Animation|PlayAnimMontage "/Game/Rod3nt/Soldiers/HumanV5/Base/AM_baseStun.AM_baseStun" 1.0 "None")))

(event Custom|Death
  (bind _mesh (Variables|Character|GetMesh))
  (Utilities|FlowControl|DoOnce false
    (:Completed
      (Development|SetHiddeninGame (Variables|Default|GetWidgetDetect) true false)
      (Collision|SetCollisionProfileName _mesh "Ragdoll" true :!class /Script/Engine.PrimitiveComponent)
      (AI|Components|Blackboard|SetValueasBool (AI|GetBlackboard (Pawn|GetController)) (Utilities|Name|MakeLiteralName "Stunned?") true)
      (Class|BINewAi|UIOff(Message) (AI|GetAIController 0))
      (Physics|SetSimulatePhysics _mesh true)
      (Components|Activation|Deactivate (Variables|Default|GetHot%20Mouth))
      (Rendering|Material|SetMaterial (Variables|Character|GetMesh) 1 "/Game/Rod3nt/Soldiers/humantest/MI_FaceDead_Inst.MI_FaceDead_Inst")
      (Niagara|SpawnSystemAttached "/Game/Rod3nt/VFX/SoldierDeath/NS_SoldierDeath.NS_SoldierDeath" (Variables|Character|GetMesh) "None" "0, 0, 0" "0, 0, 0" "KeepRelativeOffset" false)
      (Utilities|FlowControl|Delay 4.0)
      (Actor|DestroyActor))))

(event Game|Damage|EventAnyDamage
  (params (Damage :type Float%20%28single-precision%29) (DamageType :type Damage%20Type%20Object%20Reference) (InstigatedBy :type Controller%20Object%20Reference) (DamageCauser :type Actor%20Object%20Reference))
  (if (== (Utilities|GetClass DamageType) "/Game/Rod3nt/Programming/BPI+Data/Taser.Taser_C")
    (AI|Components|Blackboard|SetValueasBool (AI|GetBlackboard (Pawn|GetController)) (Utilities|Name|MakeLiteralName "Stunned?") true)
    (Niagara|SpawnSystemAttached "/Game/Rod3nt/VFX/Stunned/NS_Stunned.NS_Stunned" (Variables|Character|GetMesh) "None" "0.000000,0.000000,200.000000" "0, 0, 0" "KeepRelativeOffset" true)
    (Animation|PlayAnimMontage "/Game/Rod3nt/Soldiers/HumanV5/Base/AM_baseStun.AM_baseStun" 1.0 "None")
    (else
      (CallFunction|Death))))

(event Collision|EventHit
  (params (MyComp :type Primitive%20Component%20Object%20Reference) (Other :type Actor%20Object%20Reference) (OtherComp :type Primitive%20Component%20Object%20Reference) (bSelfMoved :type Boolean) (HitLocation :type Vector :default "0, 0, 0") (HitNormal :type Vector :default "0, 0, 0") (NormalImpulse :type Vector :default "0, 0, 0") (Hit :type Hit%20Result%20Structure%20%28by%20ref%29)))

(event EventCharMovementOff
  (Components|Tick|SetComponentTickEnabled (Variables|Character|GetCharacterMovement) false))

(event EventFacePlayer
  (Rendering|Material|SetMaterial (Variables|Character|GetMesh) 1 "/Game/Rod3nt/Soldiers/humantest/MI_FaceNormal_Inst.MI_FaceNormal_Inst"))

(event EventCharMovementon
  (Components|Tick|SetComponentTickEnabled (Variables|Character|GetCharacterMovement) true))

(event EventFireNow
  (Game|Damage|ApplyDamage (Game|Player|GetPlayerPawn 0) 5.0 0 0))

(event EventBeginPlay
  (Rendering|Material|SetMaterial (Variables|Character|GetMesh) 1 (Utilities|Array|Get(acopy) (Variables|Default|GetFaces) (Math|Random|RandomIntegerinRange 0 1)))
  (Utilities|FlowControl|Delay 2.0)
  (Components|Activation|Activate (Variables|Default|GetHot%20Mouth) false)
  (Components|Tick|SetComponentTickEnabled (Variables|Character|GetCharacterMovement) false))

(event EventCapyUIforKill
  (Variables|Default|SetKilledAlrrady? true))

(event EventSendFlying
  (params (Launch%20Vel :type Float%20%28double-precision%29))
  (bind _mesh (Variables|Character|GetMesh))
  (Utilities|FlowControl|DoOnce false
    (:Completed
      (Development|SetHiddeninGame (Variables|Default|GetWidgetDetect) true false)
      (Collision|SetCollisionProfileName _mesh "Ragdoll" true :!class /Script/Engine.PrimitiveComponent)
      (AI|Components|Blackboard|SetValueasBool (AI|GetBlackboard (Pawn|GetController)) (Utilities|Name|MakeLiteralName "Stunned?") true)
      (Class|BINewAi|UIOff(Message) (AI|GetAIController 0))
      (Physics|SetSimulatePhysics _mesh true)
      (Components|Activation|Deactivate (Variables|Default|GetHot%20Mouth))
      (Rendering|Material|SetMaterial (Variables|Character|GetMesh) 1 "/Game/Rod3nt/Soldiers/humantest/MI_FaceDead_Inst.MI_FaceDead_Inst")
      (Niagara|SpawnSystemAttached "/Game/Rod3nt/VFX/SoldierDeath/NS_SoldierDeath.NS_SoldierDeath" (Variables|Character|GetMesh) "None" "0, 0, 0" "0, 0, 0" "KeepRelativeOffset" false)
      (Utilities|FlowControl|Delay 4.0)
      (Actor|DestroyActor))))

(event EventTurnon
  (Rendering|SetRenderCustomDepth (Variables|Character|GetMesh) true))

(event EventTurnOff
  (Rendering|SetRenderCustomDepth (Variables|Character|GetMesh) false))

(event EventDmg
  (params (Health :type Float%20%28double-precision%29))
  (bind _mesh (Variables|Character|GetMesh))
  (Utilities|FlowControl|DoOnce false
    (:Completed
      (Development|SetHiddeninGame (Variables|Default|GetWidgetDetect) true false)
      (Collision|SetCollisionProfileName _mesh "Ragdoll" true :!class /Script/Engine.PrimitiveComponent)
      (AI|Components|Blackboard|SetValueasBool (AI|GetBlackboard (Pawn|GetController)) (Utilities|Name|MakeLiteralName "Stunned?") true)
      (Class|BINewAi|UIOff(Message) (AI|GetAIController 0))
      (Physics|SetSimulatePhysics _mesh true)
      (Components|Activation|Deactivate (Variables|Default|GetHot%20Mouth))
      (Rendering|Material|SetMaterial (Variables|Character|GetMesh) 1 "/Game/Rod3nt/Soldiers/humantest/MI_FaceDead_Inst.MI_FaceDead_Inst")
      (Niagara|SpawnSystemAttached "/Game/Rod3nt/VFX/SoldierDeath/NS_SoldierDeath.NS_SoldierDeath" (Variables|Character|GetMesh) "None" "0, 0, 0" "0, 0, 0" "KeepRelativeOffset" false)
      (Utilities|FlowControl|Delay 4.0)
      (Actor|DestroyActor))))

(event EventLaunchPlayer
  (params (Vector :type Vector :default "0, 0, 0"))
  (Character|LaunchCharacter Vector true true))

(event EventFaceRandom
  (Rendering|Material|SetMaterial (Variables|Character|GetMesh) 1 (Utilities|Array|Get(acopy) (Variables|Default|GetFaces) (Math|Random|RandomIntegerinRange 0 1))))

(fn ConstructionScript)

(fn AttackthePlayer
  (bind _returnvalue (Animation|PlayAnimMontage self "/Game/Rod3nt/Soldiers/HumanV5/Base/AM_KickV5.AM_KickV5" 1.0 "None"))
  (return (+ _returnvalue 0.5)))

(fn GetThepath
  (return (Variables|Default|GetAll%20Paths)))