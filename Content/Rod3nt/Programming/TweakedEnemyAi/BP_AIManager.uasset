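; AI manager that switches RodentAIController enemies on or off depending on whether they share the player's level, above or below ground.
; Once StarttheCheck is called, a looping timer checks player height and runs AboveGround or Below over every controller.
; Matching enemies get controller tick and movement enabled; others lose both and receive a UI-off message.
; The "notAllowedToWork" blackboard key is true for active enemies, despite its name.
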(event Custom|Check%20for%20distance
  (if (> (.z (Transformation|GetActorLocation (Game|Player|GetPlayerPawn 0))) -2e+02)
    (CallFunction|AboveGround)
    (else
      (CallFunction|Below))))

(event Custom|AboveGround
  (bind _outactors (Actor|GetAllActorsOfClass "/Script/ProjectRod3ntTest.RodentAIController"))
  (for _array_element _outactors
    (if (> (.z (Transformation|GetActorLocation (Pawn|GetControlledPawn _array_element))) 0.0)
      (Actor|Tick|SetActorTickEnabled _array_element true)
      (Class|BINewAi|CharMovementon(Message) (Pawn|GetControlledPawn _array_element))
      (AI|Components|Blackboard|SetValueasBool (AI|GetBlackboard _array_element) (Utilities|Name|MakeLiteralName "notAllowedToWork") true)
      (else
        (Class|BINewAi|UITurnOff(Message) _array_element)
        (Actor|Tick|SetActorTickEnabled _array_element)
        (Class|BINewAi|CharMovementOff(Message) (Pawn|GetControlledPawn _array_element))
        (AI|Components|Blackboard|SetValueasBool (AI|GetBlackboard _array_element) (Utilities|Name|MakeLiteralName "notAllowedToWork") false)))))

(event Custom|Below
  (Development|PrintString "below")
  (bind _outactors (Actor|GetAllActorsOfClass "/Script/ProjectRod3ntTest.RodentAIController"))
  (for _array_element _outactors
    (if (> (.z (Transformation|GetActorLocation (Pawn|GetControlledPawn _array_element))) 0.0)
      (Class|BINewAi|UITurnOff(Message) _array_element)
      (Class|BINewAi|CharMovementOff(Message) (Pawn|GetControlledPawn _array_element))
      (Actor|Tick|SetActorTickEnabled _array_element)
      (AI|Components|Blackboard|SetValueasBool (AI|GetBlackboard _array_element) (Utilities|Name|MakeLiteralName "notAllowedToWork") false)
      (else
        (Class|BINewAi|CharMovementon(Message) (Pawn|GetControlledPawn _array_element))
        (Actor|Tick|SetActorTickEnabled _array_element true)
        (AI|Components|Blackboard|SetValueasBool (AI|GetBlackboard _array_element) (Utilities|Name|MakeLiteralName "notAllowedToWork") true)))))

(event EventBeginPlay)

(event Collision|EventActorBeginOverlap
  (params (OtherActor :type Actor%20Object%20Reference)))

(event EventTick
  (params (DeltaSeconds :type Float%20%28single-precision%29)))

(event EventStarttheCheck
  (Utilities|Time|SetTimerbyEvent (delegate Custom|Check%20for%20distance) 0.333 true)
  (for _array_element 0
    (AI|Components|Blackboard|SetValueasBool (AI|GetBlackboard _array_element) (Utilities|Name|MakeLiteralName "notAllowedToWork") true)))

(fn ConstructionScript)

(fn AttackthePlayer
  (return 0.0))

(fn GetThepath
  (return 0))