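; BP_newPath is a spline-based path Blueprint for enemy AI that serves world-space waypoints along a looping route.
; SplinePath returns the world location of the spline point at the current PathPoint index.
; IncrementPath advances that index and wraps it to zero after the last point, so the current point is state held on the path itself.
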(event Custom|Increment%20Path
  (bind _result (Math|Integer|IncrementInt (Variables|Default|GetPath%20Point))
    (:%20%20
      (bind _output_get (Variables|Default|SetPath%20Point _result))
      (if (>= _output_get (Spline|GetNumberOfSplinePoints (Variables|Default|GetSpline)))
        (Variables|Default|SetPath%20Point 0)))))

(fn ConstructionScript)

(fn SplinePath
  (return (Spline|GetLocationatSplinePoint (Variables|Default|GetSpline) (Variables|Default|GetPath%20Point) "World")))