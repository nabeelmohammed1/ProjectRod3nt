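; RPG-wielding enemy AI character that fires rockets at the player and can be stunned or killed.
; FireNow spawns BP_RPG from an arrow aimed at the player with random pitch and roll jitter.
; Taser damage or Stunnable overlaps set a blackboard stun flag, while other damage triggers a one-shot ragdoll death and delayed destruction.
; Events swap face materials, toggle custom-depth rendering, and switch movement ticking, which starts disabled after a delay.
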(event OnComponentBeginOverlap(Capsule)
  (params (OverlappedComponent :type Primitive%20Component%20Object%20Reference) (OtherActor :type Actor%20Object%20Reference) (OtherComp :type Primitive%20Component%20Object%20Reference) (OtherBodyIndex :type Integer) (bFromSweep :type Boolean) (SweepResult :type Hit%20Result%20Structure%20%28by%20ref%29))
  (if (Actor|ActorHasTag OtherActor "Stunnable")
    (AI|Components|Blackboard|SetValueasBool (AI|GetBlackboard (Pawn|GetController)) (Utilities|Name|MakeLiteralName "Stunned?") true)
    (Niagara|SpawnSystemAttached "/Game/Rod3nt/VFX/Stunned/NS_Stunned.NS_Stunned" (Variables|Character|GetMesh) "None" "0.000000,0.000000,200.000000" "0, 0, 0" "KeepRelativeOffset" true)
    (Animation|PlayAnimMontage "/Game/Rod3nt/Soldiers/HumanV5/RPG/AM_RpgStun.AM_RpgStun" 1.0 "None")))

(event Custom|Death
  (bind _mesh (Variables|Character|GetMesh))
  (Utilities|FlowControl|DoOnce false
    (:Completed
      (Development|SetHiddeninGame (Variables|Default|GetWidgetDetect) true false)
      (Collision|SetCollisionProfileName _mesh "Ragdoll" true :!class /Script/Engine.PrimitiveComponent)
      (AI|Components|Blackboard|SetValueasBool (AI|GetBlackboard (Pawn|GetController)) (Utilities|Name|MakeLiteralName "Stunned?") true)
      (Class|BINewAi|UIOff(Message) (AI|GetAIController 0))
      (Physics|SetSimulatePhysics _mesh true)
      (Components|Activation|Deactivate (Variables|Default|GetHotMouth))
      (Niagara|SpawnSystemAttached "/Game/Rod3nt/VFX/SoldierDeath/NS_SoldierDeath.NS_SoldierDeath" (Variables|Character|GetMesh) "None" "0, 0, 0" "0, 0, 0" "KeepRelativeOffset" false)
      (Utilities|FlowControl|Delay 4.0)
      (Actor|DestroyActor))))

(event Game|Damage|EventAnyDamage
  (params (Damage :type Float%20%28single-precision%29) (DamageType :type Damage%20Type%20Object%20Reference) (InstigatedBy :type Controller%20Object%20Reference) (DamageCauser :type Actor%20Object%20Reference))
  (if (== (Utilities|GetClass DamageType) "/Game/Rod3nt/Programming/BPI+Data/Taser.Taser_C")
    (AI|Components|Blackboard|SetValueasBool (AI|GetBlackboard (Pawn|GetController)) (Utilities|Name|MakeLiteralName "Stunned?") true)
    (Niagara|SpawnSystemAttached "/Game/Rod3nt/VFX/Stunned/NS_Stunned.NS_Stunned" (Variables|Character|GetMesh) "None" "0.000000,0.000000,200.000000" "0, 0, 0" "KeepRelativeOffset" true)
    (Animation|PlayAnimMontage "/Game/Rod3nt/Soldiers/HumanV5/RPG/AM_RpgStun.AM_RpgStun" 1.0 "None")
    (else
      (CallFunction|Death)
      (Rendering|Material|SetMaterial (Variables|Character|GetMesh) 2 "/Game/Rod3nt/Soldiers/humantest/MI_FaceDead_Inst.MI_FaceDead_Inst"))))

(event Collision|EventHit
  (params (MyComp :type Primitive%20Component%20Object%20Reference) (Other :type Actor%20Object%20Reference) (OtherComp :type Primitive%20Component%20Object%20Reference) (bSelfMoved :type Boolean) (HitLocation :type Vector :default "0, 0, 0") (HitNormal :type Vector :default "0, 0, 0") (NormalImpulse :type Vector :default "0, 0, 0") (Hit :type Hit%20Result%20Structure%20%28by%20ref%29)))

(event EventFaceRandom
  (Rendering|Material|SetMaterial (Variables|Character|GetMesh) 2 (Utilities|Array|Get(acopy) (Variables|Default|GetFaces) (Math|Random|RandomIntegerinRange 0 1))))

(event EventFacePlayer
  (Rendering|Material|SetMaterial (Variables|Character|GetMesh) 2 "/Game/Rod3nt/Soldiers/humantest/MI_FaceNormal_Inst.MI_FaceNormal_Inst"))

(event EventCharMovementOff
  (Components|Tick|SetComponentTickEnabled (Variables|Character|GetCharacterMovement) false))

(event EventCharMovementon
  (Components|Tick|SetComponentTickEnabled (Variables|Character|GetCharacterMovement) true))

(event EventBeginPlay
  (Rendering|Material|SetMaterial (Variables|Character|GetMesh) 2 (Utilities|Array|Get(acopy) (Variables|Default|GetFaces) (Math|Random|RandomIntegerinRange 0 1)))
  (Utilities|FlowControl|Delay 2.0)
  (Components|Activation|Activate (Variables|Default|GetHotMouth) false)
  (Components|Tick|SetComponentTickEnabled (Variables|Character|GetCharacterMovement) false))

(event EventFireNow
  (bind _returnvalue (Math|Random|RandomFloatinRange -3.0 3.0))
  (bind _returnvalue_2 (Game|Player|GetPlayerPawn 0))
  (bind _arrow1 (Variables|Default|GetArrow1))
  (bind _arrow1_2 (Variables|Default|GetArrow1))
  (bind _returnvalue_3 (Transformation|GetActorLocation _returnvalue_2))
  (bind _returnvalue_4 (Transformation|GetWorldLocation _arrow1))
  (bind _returnvalue_5 (Transformation|GetWorldLocation _arrow1_2))
  (bind _returnvalue_6 (Math|Rotator|FindLookatRotation _returnvalue_4 _returnvalue_3))
  (Transformation|SetWorldRotation (Variables|Default|GetArrow1) (Math|Rotator|MakeRotator (+ (.roll _returnvalue_6) _returnvalue) (+ (.pitch _returnvalue_6) _returnvalue) (.yaw _returnvalue_6)) false false)
  (Game|SpawnActorfromClass "/Game/Rod3nt/Programming/PICKUPSandENVI-BPS/BP_RPG.BP_RPG_C" (Math|Transform|MakeTransform _returnvalue_5 (Transformation|GetWorldRotation _arrow1_2) "1.000000,1.000000,1.000000") "Undefined" "MultiplyWithRoot" 0 0)
  (Audio|PlaySoundatLocation "/Game/Rod3nt/sounds/TankShot2.TankShot2" _returnvalue_5 "0, 0, 0" 1.0 1.0 0.0 "/Game/Rod3nt/sounds/gunshot1.gunshot1" 0 0 0)
  (Niagara|SpawnSystematLocation "/Game/Rod3nt/VFX/MuzzleFlash/NS_MuzzleFlash.NS_MuzzleFlash" (Transformation|GetWorldLocation (Variables|Default|GetArrow1))))

(event EventTurnOff
  (Rendering|SetRenderCustomDepth (Variables|Character|GetMesh) false))

(event EventTurnon
  (Rendering|SetRenderCustomDepth (Variables|Character|GetMesh) true))

(event EventSendFlying
  (params (Launch%20Vel :type Float%20%28double-precision%29))
  (bind _mesh (Variables|Character|GetMesh))
  (Utilities|FlowControl|DoOnce false
    (:Completed
      (Development|SetHiddeninGame (Variables|Default|GetWidgetDetect) true false)
      (Collision|SetCollisionProfileName _mesh "Ragdoll" true :!class /Script/Engine.PrimitiveComponent)
      (AI|Components|Blackboard|SetValueasBool (AI|GetBlackboard (Pawn|GetController)) (Utilities|Name|MakeLiteralName "Stunned?") true)
      (Class|BINewAi|UIOff(Message) (AI|GetAIController 0))
      (Physics|SetSimulatePhysics _mesh true)
      (Components|Activation|Deactivate (Variables|Default|GetHotMouth))
      (Niagara|SpawnSystemAttached "/Game/Rod3nt/VFX/SoldierDeath/NS_SoldierDeath.NS_SoldierDeath" (Variables|Character|GetMesh) "None" "0, 0, 0" "0, 0, 0" "KeepRelativeOffset" false)
      (Utilities|FlowControl|Delay 4.0)
      (Actor|DestroyActor))))

(event EventLaunchPlayer
  (params (Vector :type Vector :default "0, 0, 0"))
  (Character|LaunchCharacter Vector true true))

(event EventDmg
  (params (Health :type Float%20%28double-precision%29))
  (CallFunction|Death)
  (Rendering|Material|SetMaterial (Variables|Character|GetMesh) 2 "/Game/Rod3nt/Soldiers/humantest/MI_FaceDead_Inst.MI_FaceDead_Inst"))

(event EventCapyUIforKill
  (Variables|Default|SetKilledAlrrady? true))

(fn ConstructionScript)

(fn AttackthePlayer
  (bind _returnvalue (Animation|PlayAnimMontage "/Game/Rod3nt/Soldiers/HumanV5/RPG/AM_RpgFireV5.AM_RpgFireV5" 1.0 "None"))
  (return (+ _returnvalue 2.0)))

(fn GetThepath
  (return (Variables|Default|GetAll%20Paths)))