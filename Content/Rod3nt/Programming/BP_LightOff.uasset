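; BP_LightOff is an actor that knocks out nearby spotlights and weakens rodent AI vision around it.
; SendFlying sets DisableSight and zeroes the intensity of every SpotLight within the SearchForLight sphere, found by a distance check.
; Once flagged, EnemyCollider overlaps temporarily reduce vision on BI_newAi actors' RodentAIController and restore it on exit.
; ResetLights relights those spotlights, but its timer is unconnected and DisableSight is never cleared.
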(event OnComponentBeginOverlap(SearchForLight)
  (params (OverlappedComponent :type Primitive%20Component%20Object%20Reference) (OtherActor :type Actor%20Object%20Reference) (OtherComp :type Primitive%20Component%20Object%20Reference) (OtherBodyIndex :type Integer) (bFromSweep :type Boolean) (SweepResult :type Hit%20Result%20Structure%20%28by%20ref%29)))

(event OnComponentBeginOverlap(EnemyCollider)
  (params (OverlappedComponent :type Primitive%20Component%20Object%20Reference) (OtherActor :type Actor%20Object%20Reference) (OtherComp :type Primitive%20Component%20Object%20Reference) (OtherBodyIndex :type Integer) (bFromSweep :type Boolean) (SweepResult :type Hit%20Result%20Structure%20%28by%20ref%29))
  (if (Variables|Default|GetDisable%20Sight)
    (if (Utilities|DoesObjectImplementInterface OtherActor "/Game/Rod3nt/Programming/TweakedEnemyAi/BI_newAi.BI_newAi_C")
      (bind _asrodent_aicontroller (Utilities|Casting|CastToRodentAIController (AI|GetAIController OtherActor)))
      (Class|RodentAIController|ReduceVisionTemporaily _asrodent_aicontroller 45.0 6e+02))))

(event OnComponentEndOverlap(EnemyCollider)
  (params (OverlappedComponent :type Primitive%20Component%20Object%20Reference) (OtherActor :type Actor%20Object%20Reference) (OtherComp :type Primitive%20Component%20Object%20Reference) (OtherBodyIndex :type Integer))
  (if (Variables|Default|GetDisable%20Sight)
    (if (Utilities|DoesObjectImplementInterface OtherActor "/Game/Rod3nt/Programming/TweakedEnemyAi/BI_newAi.BI_newAi_C")
      (bind _asrodent_aicontroller (Utilities|Casting|CastToRodentAIController (AI|GetAIController OtherActor)))
      (Class|RodentAIController|RestoreVisiontoNormal _asrodent_aicontroller))))

(event Custom|Look%20Fior%20Light
  (bind _search_for_light (Variables|Default|GetSearch%20For%20Light))
  (Variables|Default|SetDisable%20Sight true)
  (Development|PrintString "sifghgt reduction" true true "(R=0.628096,G=0.388576,B=1.000000,A=1.000000)")
  (bind _outactors (Actor|GetAllActorsOfClass "/Script/Engine.SpotLight"))
  (for _array_element _outactors
    (if (<= (Math|Vector|Distance(Vector) (Transformation|GetActorLocation _array_element) (Transformation|GetWorldLocation _search_for_light)) (Components|Sphere|GetScaledSphereRadius _search_for_light))
      (bind _asspot_light (Utilities|Casting|CastToSpotLight _array_element))
      (Rendering|Components|Light|SetIntensity (Variables|/Script/Engine.SpotLight|GetSpotLightComponent _asspot_light) 0.0))))

(event Custom|Reset%20Lights
  (bind _search_for_light (Variables|Default|GetSearch%20For%20Light))
  (bind _outactors (Actor|GetAllActorsOfClass "/Script/Engine.SpotLight"))
  (for _array_element _outactors
    (if (<= (Math|Vector|Distance(Vector) (Transformation|GetActorLocation _array_element) (Transformation|GetWorldLocation _search_for_light)) (Components|Sphere|GetScaledSphereRadius _search_for_light))
      (bind _asspot_light (Utilities|Casting|CastToSpotLight _array_element))
      (Rendering|Components|Light|SetIntensity (Variables|/Script/Engine.SpotLight|GetSpotLightComponent _asspot_light) 15.0))))

(event EventBeginPlay)

(event Collision|EventActorBeginOverlap
  (params (OtherActor :type Actor%20Object%20Reference)))

(event EventSendFlying
  (params (Launch%20Vel :type Float%20%28double-precision%29))
  (CallFunction|LookFiorLight))

(fn ConstructionScript)