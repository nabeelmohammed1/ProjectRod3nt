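; An EQS context that supplies the querier's current attack target as a single actor for environment queries.
; It gets the querier's AI controller, casts it and returns its AttackTargetReference.
; It also carries empty stub functions for attack, path, target, range, mesh and movement speed, which return nothing or zero.
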(fn ProvideSingleActor
  (params (QuerierObject :type Object%20Object%20Reference) (QuerierActor :type Actor%20Object%20Reference))
  (bind _asaic_ai (Utilities|Casting|CastTo (AI|GetAIController QuerierActor)))
  (return (Variables|Default|GetAttack%20Target%20Reference _asaic_ai)))

(fn AIAttack
  (return 0))

(fn AIPath
  (return 0))

(fn AttackTarget
  (return 0))

(fn GetIdealRange
  (return 0.0 0.0))

(fn GetmyMesh
  (return 0))

(fn MovementSpeed
  (params (Speed :type E_MovementSpeed%20Enum :default "NewEnumerator0"))
  (return 0.0))