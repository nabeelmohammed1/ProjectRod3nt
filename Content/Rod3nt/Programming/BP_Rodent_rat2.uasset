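; Rodent rat character Blueprint that extends its parent with stealth crouching, a spawn glider and a death effect.
; Releasing IA_Crouch toggles crouch, changing walk speed, Cube collision, gameplay tags and taser spawner height.
; Crouching also unregisters the AI perception source and clears TargetActor on every RodentAIController blackboard, while standing re-registers for sight.
; During spawn glide, the glider yaw follows the camera and hides on landing.
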(event Input|EnhancedActionEvents|EnhancedInputActionIA_Crouch
  (params (ActionValue :type Vector%202D%20Structure) (ElapsedSeconds :type Float%20%28double-precision%29) (TriggeredSeconds :type Float%20%28double-precision%29) (InputAction :type Input%20Action%20Object%20Reference :default "/Game/Input/Actions/IA_Crouch.IA_Crouch"))
  (bind _self self)
  (bind _charactermovement (Variables|Character|GetCharacterMovement))
  (bind _gameplaytags (Variables|Default|GetGameplayTags))
  (bind _aiperceptionstimulisource (Variables|Default|GetAIPerceptionStimuliSource))
  (bind _rotating_taser_spawner (Variables|Default|GetRotating%20Taser%20Spawner))
  (:Completed
    (Utilities|FlowControl|FlipFlop
      (:A
        (Variables|Default|Setcoruching? true)
        (Variables|/Script/Engine.CharacterMovementComponent|SetMaxWalkSpeed _charactermovement (Variables|Default|GetMovementSpeedCrouching))
        (Collision|SetCollisionEnabled (Variables|Default|GetCube) "QueryAndPhysics")
        (Development|PrintString "crouch")
        (Class|AIPerceptionStimuliSourceComponent|UnregisterfromPerceptionSystem _aiperceptionstimulisource)
        (Ability|GameplayEffect|AddLooseGameplayTags _self _gameplaytags)
        (Transformation|SetRelativeLocation _rotating_taser_spawner "0.000000,0.436370,-0.040526" false false)
        (bind _outactors (Actor|GetAllActorsOfClass "/Script/ProjectRod3ntTest.RodentAIController"))
        (for _array_element _outactors
          (AI|Components|Blackboard|SetValueasObject (AI|GetBlackboard _array_element) (Utilities|Name|MakeLiteralName "TargetActor") 0)))
      (:B
        (Variables|Default|Setcoruching? false)
        (bind _output_get (Variables|/Script/Engine.CharacterMovementComponent|SetMaxWalkSpeed _charactermovement (Variables|Default|Getdefault%20Walk%20Speed)))
        (Collision|SetCollisionEnabled (Variables|Default|GetCube) "NoCollision")
        (Variables|Default|SetResetWalkSpeed _output_get)
        (Development|PrintString "no crouch")
        (Class|AIPerceptionStimuliSourceComponent|RegisterforSense _aiperceptionstimulisource "/Script/AIModule.AISense_Sight")
        (Ability|GameplayEffect|RemoveLooseGameplayTags _self _gameplaytags)
        (Transformation|SetRelativeLocation _rotating_taser_spawner "0.000000,0.436370,0.300000" false false)))))

(event EventBeginPlay
  (|CallParentFunction)
  (Collision|SetCollisionEnabled (Variables|Default|GetCube) "NoCollision")
  (if (Variables|Default|GetbStartwithSpawnGlide)
    (Rendering|SetVisibility (Variables|Default|GetGlider) true false)))

(event Collision|EventActorBeginOverlap
  (params (OtherActor :type Actor%20Object%20Reference))
  (|CallParentFunction OtherActor) ; This node is disabled and will not be called.\nDrag off pins to build functionality.
)

(event EventOnLanded
  (params (Hit :type Hit%20Result%20Structure%20%28by%20ref%29))
  (if (Variables|Default|GetbIsSpawnGliding)
    (Rendering|SetVisibility (Variables|Default|GetGlider) false false))
  (|CallParentFunction Hit))

(event EventTick
  (params (DeltaSeconds :type Float%20%28single-precision%29))
  (|CallParentFunction 0.0))

(event EventDeathVFX
  (bind _ded (Variables|Default|GetDed))
  (Development|PrintString (Utilities|String|ToString(Boolean) (Utilities|IsValid _ded)))
  (Components|Activation|Activate _ded true))

(fn ConstructionScript
  (|CallParentFunction))

(fn Aim
  (params (X%20Axis :type Float%20%28single-precision%29) (Y%20Axis :type Float%20%28double-precision%29))
  (|CallParentFunction X%20Axis Y%20Axis)
  (if (Variables|Default|GetbIsSpawnGliding)
    (Transformation|SetRelativeRotation (Variables|Default|GetGlider) (Math|Rotator|MakeRotator 0.0 0.0 (Math|Rotator|NormalizeAxis (+ (- (.Yaw (Math|Rotator|BreakRotator (Transformation|GetWorldRotation (Variables|Default|GetCamera)))) (.Yaw (Math|Rotator|BreakRotator (Transformation|GetActorRotation)))) -1.8e+02))) true true)))