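; Squirrel rodent character Blueprint that builds on a parent class, adding a camera pitch limit and a death effect.
; On BeginPlay it runs the parent logic, then clamps the first player camera manager's view pitch.
; DeathVFX prints a validity check and activates the Ded component.
; Overlap, landing, tick and construction only call the parent, and leftover glide, spring arm and dash Niagara nodes are unwired.
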(event EventBeginPlay
  (|CallParentFunction)
  (CallFunction|CameraLock))

(event Collision|EventActorBeginOverlap
  (params (OtherActor :type Actor%20Object%20Reference))
  (|CallParentFunction OtherActor))

(event EventTick
  (params (DeltaSeconds :type Float%20%28single-precision%29))
  (|CallParentFunction DeltaSeconds))

(event EventOnLanded
  (params (Hit :type Hit%20Result%20Structure%20%28by%20ref%29))
  (|CallParentFunction Hit))

(event EventDeathVFX
  (bind _ded (Variables|Default|GetDed))
  (Development|PrintString (Utilities|String|ToString(Boolean) (Utilities|IsValid _ded)))
  (Components|Activation|Activate _ded true))

(event EventCameraLock
  (bind _returnvalue (Game|GetPlayerCameraManager 0))
  ;[0.15 0.15 0.15 0.5] Camera
  (Variables|/Script/Engine.PlayerCameraManager|SetViewPitchMax _returnvalue 2e+01)
  (Variables|/Script/Engine.PlayerCameraManager|SetViewPitchMin _returnvalue -3e+01))

(fn ConstructionScript
  (|CallParentFunction))