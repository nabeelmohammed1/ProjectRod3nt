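; Tutorial exit teleporter that starts the main game by loading newMainLevel when its trigger box is overlapped.
; On BeginPlay it briefly hides its spotlight, then shows it again.
; Any overlap reveals the lights and cylinder, plays sounds, destroys the box, then after timed delays adds a fade widget before opening the level.
; Disconnected leftovers include a looping gliding sound and an unused player pawn lookup.
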(event OnComponentBeginOverlap(Box)
  (params (OverlappedComponent :type Primitive%20Component%20Object%20Reference) (OtherActor :type Actor%20Object%20Reference) (OtherComp :type Primitive%20Component%20Object%20Reference) (OtherBodyIndex :type Integer) (bFromSweep :type Boolean) (SweepResult :type Hit%20Result%20Structure%20%28by%20ref%29))
  (bind _output_get (Variables|Default|SetTeleporterOn true))
  (Rendering|SetVisibility (Variables|Default|GetPointLight) true false)
  (Rendering|SetVisibility (Variables|Default|GetCylinder) true false)
  (Rendering|SetVisibility (Variables|Default|GetSpotLight) true false)
  (Audio|PlaySoundatLocation "/Game/Rod3nt/sounds/Ui/teleporterSound.teleporterSound" (Transformation|GetWorldLocation (Variables|Default|GetDefaultSceneRoot)) "0, 0, 0" 1.0 1.0 0.0 0 0 0 0)
  (if (Variables|Default|GetTeleporterOn)
    (if _output_get
      (Audio|PlaySound2D "/Game/Rod3nt/sounds/Ui/UI-Sound-6.UI-Sound-6" 1.0 1.0 0.0 0 0)
      (Components|DestroyComponent (Variables|Default|GetBox))
      (Utilities|FlowControl|DoOnce false
        (:Completed
          (Utilities|FlowControl|Delay 5.0)
          (bind _returnvalue (UserInterface|CreateWidget "/Game/Rod3nt/Programming/UI/WBP_Fade.WBP_Fade_C"))
          (UserInterface|Viewport|AddtoViewport _returnvalue 0)
          (Utilities|FlowControl|Delay 1.0)
          (Game|OpenLevel(byName) "newMainLevel"))))))

(event EventBeginPlay
  (Rendering|SetVisibility (Variables|Default|GetSpotLight) false false)
  (Utilities|FlowControl|Delay 1.0)
  (Rendering|SetVisibility (Variables|Default|GetSpotLight) true false))

(fn ConstructionScript)