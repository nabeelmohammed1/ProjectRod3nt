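; BP_DeadSquirrel is a dead squirrel actor that relies on its parent class for behavior.
; On BeginPlay it runs the parent logic, then raises its skeletal mesh 15 units in world Z.
; The runtime offset works around the mesh not being movable in the viewport.
; Overlap and Tick events are disabled stubs, and the construction script only calls the parent.
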(event EventBeginPlay
  (bind _skeletalmesh (Variables|Default|GetSkeletalMesh))
  (|CallParentFunction)
  ;[0.15 0.15 0.15 0.5] Can't change and move the SKM in viewport,
  (Transformation|SetWorldLocation _skeletalmesh (+ (Transformation|GetWorldLocation _skeletalmesh) "0.000000,0.000000,15.000000") false false))

(event Collision|EventActorBeginOverlap
  (params (OtherActor :type Actor%20Object%20Reference))
  (|CallParentFunction OtherActor) ; This node is disabled and will not be called.\nDrag off pins to build functionality.
)

(event EventTick
  (params (DeltaSeconds :type Float%20%28single-precision%29))
  (|CallParentFunction DeltaSeconds) ; This node is disabled and will not be called.\nDrag off pins to build functionality.
)

(fn ConstructionScript
  (|CallParentFunction))