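; BP_DeadMaster is a dead rodent the player can absorb to gain health, walk speed, jump and climb boosts.
; An overlap box shows or hides an interact widget for the rat player.
; Interacting inside it freezes movement, plays a Niagara download effect linking the corpse and player meshes, and sends the boosts through DownloadStatsMessage.
; After a delay it restores movement, removes the widget and destroys itself.
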(event OnComponentBeginOverlap(Box)
  (params (OverlappedComponent :type Primitive%20Component%20Object%20Reference) (OtherActor :type Actor%20Object%20Reference) (OtherComp :type Primitive%20Component%20Object%20Reference) (OtherBodyIndex :type Integer) (bFromSweep :type Boolean) (SweepResult :type Hit%20Result%20Structure%20%28by%20ref%29))
  (if (Variables|Default|Getcan%20work?)
    (if (Utilities|DoesObjectImplementInterface OtherActor "/Game/Rod3nt/Programming/BPI+Data/BI_PlayeRat.BI_PLayeRat_C")
      (Variables|/Script/UMG.Widget|SetVisibility (Variables|Default|GetWidget) "Visible"))))

(event OnComponentEndOverlap(Box)
  (params (OverlappedComponent :type Primitive%20Component%20Object%20Reference) (OtherActor :type Actor%20Object%20Reference) (OtherComp :type Primitive%20Component%20Object%20Reference) (OtherBodyIndex :type Integer))
  (if (Variables|Default|Getcan%20work?)
    (if (Utilities|DoesObjectImplementInterface OtherActor "/Game/Rod3nt/Programming/BPI+Data/BI_PlayeRat.BI_PLayeRat_C")
      (Variables|/Script/UMG.Widget|SetVisibility (Variables|Default|GetWidget) "Hidden"))))

(event Input|EnhancedActionEvents|EnhancedInputActionIA_Interact1
  (params (ActionValue :type Boolean) (ElapsedSeconds :type Float%20%28double-precision%29) (TriggeredSeconds :type Float%20%28double-precision%29) (InputAction :type Input%20Action%20Object%20Reference :default "/Game/Input/Actions/IA_Interact1.IA_Interact1"))
  (bind _returnvalue (Game|GetPlayerCharacter 0))
  (bind _returnvalue_2 (Game|GetPlayerCharacter 0))
  (bind _returnvalue_3 (Game|GetPlayerCharacter 0))
  (bind _skeletalmesh (Variables|Default|GetSkeletalMesh))
  (bind _mesh (Variables|/Script/Engine.Character|GetMesh _returnvalue_2))
  (bind _charactermovement (Variables|/Script/Engine.Character|GetCharacterMovement _returnvalue))
  (:Completed
    (if (Collision|IsOverlappingActor (Variables|Default|GetBox) _returnvalue_3 :!class /Script/Engine.PrimitiveComponent)
      (Utilities|IsValid _skeletalmesh
        (:Is%20Valid
          (Utilities|FlowControl|DoOnce false
            (:Completed
              (Input|SetIgnoreMoveInput (Game|GetPlayerController 0) true)
              (Components|Movement|StopMovementImmediately _charactermovement)
              (Pawn|Components|CharacterMovement|DisableMovement _charactermovement)
              (bind _returnvalue_4 (Niagara|SpawnSystemAttached "/Game/Rod3nt/VFX/Download/NS_Download.NS_Download" _skeletalmesh "None" (Transformation|GetWorldLocation _skeletalmesh) "0, 0, 0" "KeepWorldPosition" false))
              (Class|NiagaraFunctionLibrary|OverrideSystemUserVariableSkeletalMeshComponent _returnvalue_4 "DeadPawn" _skeletalmesh)
              (Class|NiagaraFunctionLibrary|OverrideSystemUserVariableSkeletalMeshComponent _returnvalue_4 "CurrentPawn" _mesh)
              (Niagara|SetNiagaraVariable(Vector3) _returnvalue_4 "User.AbsorptionLOC" (Transformation|GetSocketLocation _mesh "rootSocket"))
              (Class|BIPLayeRat|DownloadStats(Message) _returnvalue_3 (Variables|Default|GetHealthBoost) (Variables|Default|GetWalkSpeedBoost) (Variables|Default|GetJumpBoost) (Variables|Default|GetClimbBoost))
              ;[0.15 0.15 0.15 0.5] Originally .2
              (Utilities|FlowControl|Delay 3.0)
              (Input|SetIgnoreMoveInput (Game|GetPlayerController 0) false)
              (Pawn|Components|CharacterMovement|SetMovementMode (Variables|/Script/Engine.Character|GetCharacterMovement (Game|GetPlayerCharacter 0)) "MOVE_Walking" 0)
              (Widget|RemovefromParent (stale EventBeginPlay _returnvalue_2))
              (Actor|DestroyActor))))))))

(event EventBeginPlay
  (bind _returnvalue (Game|GetPlayerController 0))
  (Utilities|FlowControl|Delay 2.0)
  (Variables|Default|Setcan%20work? true)
  (Input|EnableInput _returnvalue)
  (bind _returnvalue_2 (UserInterface|CreateWidget "/Game/Rod3nt/Programming/UI/WBP_Interact.WBP_Interact_C" _returnvalue))
  (Variables|Default|SetWidget _returnvalue_2)
  (UserInterface|Viewport|AddtoViewport _returnvalue_2 0)
  (Variables|/Script/UMG.Widget|SetVisibility _returnvalue_2 "Hidden"))

(fn ConstructionScript)