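; BP_GunFallKill is a trigger actor that starts a cutscene, apparently a gun-fall kill, once the boss is in position.
; Its CutsceneStarter volume has collision off at BeginPlay and is query-only while an actor tagged Boss overlaps BossDetector.
; When an actor implementing BI_Utli enters the armed volume, it calls CutsceneTie on BP_KillGuy2 and sends a sequence-type message to the GameInstance.
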(event OnComponentBeginOverlap(BossDetector)
  (params (OverlappedComponent :type Primitive%20Component%20Object%20Reference) (OtherActor :type Actor%20Object%20Reference) (OtherComp :type Primitive%20Component%20Object%20Reference) (OtherBodyIndex :type Integer) (bFromSweep :type Boolean) (SweepResult :type Hit%20Result%20Structure%20%28by%20ref%29))
  (if (Actor|ActorHasTag OtherActor "Boss")
    (Collision|SetCollisionEnabled (Variables|Default|GetCutsceneStarter) "QueryOnly")))

(event OnComponentBeginOverlap(CutsceneStarter)
  (params (OverlappedComponent :type Primitive%20Component%20Object%20Reference) (OtherActor :type Actor%20Object%20Reference) (OtherComp :type Primitive%20Component%20Object%20Reference) (OtherBodyIndex :type Integer) (bFromSweep :type Boolean) (SweepResult :type Hit%20Result%20Structure%20%28by%20ref%29))
  (if (Utilities|DoesObjectImplementInterface OtherActor "/Game/Rod3nt/Programming/BPI+Data/BI_Utli.BI_Utli_C")
    (bind _returnvalue (Actor|GetActorOfClass "/Game/Rod3nt/Programming/BP_KillGuy2.BP_KillGuy2_C"))
    (Default|CutsceneTie _returnvalue)
    (Class|BIGI|SequenceType(Message) (Game|GetGameInstance) "NewEnumerator5")))

(event OnComponentEndOverlap(BossDetector)
  (params (OverlappedComponent :type Primitive%20Component%20Object%20Reference) (OtherActor :type Actor%20Object%20Reference) (OtherComp :type Primitive%20Component%20Object%20Reference) (OtherBodyIndex :type Integer))
  (if (Actor|ActorHasTag OtherActor "Boss")
    (Collision|SetCollisionEnabled (Variables|Default|GetCutsceneStarter) "NoCollision")))

(event EventBeginPlay
  (Collision|SetCollisionEnabled (Variables|Default|GetCutsceneStarter) "NoCollision"))

(fn ConstructionScript)