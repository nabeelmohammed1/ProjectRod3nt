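; BP_Sun is a Blueprint that tracks the player's death and underground state and shows the lose screen when the game is lost.
; Player death, spawn and ground-crossing events set the HasDied and IsUnderground flags, with spawning clearing both.
; OnGameLost creates WBP_LoseScreen, adds it to the viewport and gives it focus.
; Tick and the construction script are empty, and a debug print of CurrentMin is disconnected.
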(event EventTick
  (params (DeltaSeconds :type Float%20%28single-precision%29))
  ;[0.15 0.15 0.15 0.5] 1080 was prev
)

(event EventPlayerDied
  (Variables|Default|SetbHasDied true))

(event EventOnGameLost
  (bind _returnvalue (UserInterface|CreateWidget "/Game/Rod3nt/Programming/UI/WBP_LoseScreen.WBP_LoseScreen_C"))
  (UserInterface|Viewport|AddtoViewport _returnvalue 0)
  (Widget|SetFocus _returnvalue))

(event EventPlayerSpawned
  (Variables|Default|SetbHasDied false)
  (Variables|Default|SetbIsUnderground false))

(event EventBelowGround
  (Variables|Default|SetbIsUnderground true))

(event EventAboveGround
  (Variables|Default|SetbIsUnderground false))

(fn ConstructionScript)