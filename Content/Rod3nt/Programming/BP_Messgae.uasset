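; BP_Messgae is a trigger actor for a message spot that awards the "Dev_Love" achievement and briefly takes over the player's view.
; Any Box overlap disables pawn input, calls the game instance's achievement function and blends the view to this actor.
; After a short delay it restores input and blends back to the pawn, with no once-only guard.
; An unconnected Timeline chain that would rotate the player's view toward the Decal never runs.
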(event OnComponentBeginOverlap(Box)
  (params (OverlappedComponent :type Primitive%20Component%20Object%20Reference) (OtherActor :type Actor%20Object%20Reference) (OtherComp :type Primitive%20Component%20Object%20Reference) (OtherBodyIndex :type Integer) (bFromSweep :type Boolean) (SweepResult :type Hit%20Result%20Structure%20%28by%20ref%29))
  (bind _returnvalue (Game|GetPlayerController 0))
  (bind _returnvalue_2 (Game|Player|GetPlayerPawn 0))
  (Input|DisableInput (Game|Player|GetPlayerPawn 0) _returnvalue)
  (Class|BIGI|AchievmentType(Message) (Game|GetGameInstance) "Dev_Love" 1.0)
  (Game|Player|SetViewTargetwithBlend _returnvalue self 1.0 "VTBlend_EaseIn" 0.0 false)
  (Utilities|FlowControl|Delay 2.0)
  (Input|EnableInput _returnvalue_2 _returnvalue)
  (Game|Player|SetViewTargetwithBlend _returnvalue _returnvalue_2 1.0 "VTBlend_EaseIn" 0.0 false))

(fn ConstructionScript)