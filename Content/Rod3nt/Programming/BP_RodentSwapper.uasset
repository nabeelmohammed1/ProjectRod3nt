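; BP_RodentSwapper is an interactable station that activates a Gameplay Ability, presumably a rodent swap, on the player character.
; Its Box trigger toggles a WBP_RodentSwap widget for BI_PLayeRat actors.
; The first overlap sends a Capy UI message and clears FirstTime on every swapper instance, so the message is not repeated.
; IA_Interact1 inside the box grants and activates AbilityClass once through GAS and plays a sound at the mesh.
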(event OnComponentBeginOverlap(Box)
  (params (OverlappedComponent :type Primitive%20Component%20Object%20Reference) (OtherActor :type Actor%20Object%20Reference) (OtherComp :type Primitive%20Component%20Object%20Reference) (OtherBodyIndex :type Integer) (bFromSweep :type Boolean) (SweepResult :type Hit%20Result%20Structure%20%28by%20ref%29))
  (if (Utilities|DoesObjectImplementInterface OtherActor "/Game/Rod3nt/Programming/BPI+Data/BI_PlayeRat.BI_PLayeRat_C")
    (Variables|/Script/UMG.Widget|SetVisibility (Variables|Default|GetUI) "Visible")
    (if (Variables|Default|GetFirst%20Time?)
      (Class|BIPLayeRat|UIforCapy(Message) OtherActor "NewEnumerator1")
      (Variables|Default|SetFirst%20Time? false)
      (bind _outactors (Actor|GetAllActorsOfClass "BP_RodentSwapper_C"))
      (for _array_element _outactors
        (Variables|BP_RodentSwapper_C|SetFirst%20Time? _array_element false)))))

(event OnComponentEndOverlap(Box)
  (params (OverlappedComponent :type Primitive%20Component%20Object%20Reference) (OtherActor :type Actor%20Object%20Reference) (OtherComp :type Primitive%20Component%20Object%20Reference) (OtherBodyIndex :type Integer))
  (if (Utilities|DoesObjectImplementInterface OtherActor "/Game/Rod3nt/Programming/BPI+Data/BI_PlayeRat.BI_PLayeRat_C")
    (Variables|/Script/UMG.Widget|SetVisibility (Variables|Default|GetUI) "Hidden")))

(event Input|EnhancedActionEvents|EnhancedInputActionIA_Interact1
  (params (ActionValue :type Vector%202D%20Structure) (ElapsedSeconds :type Float%20%28double-precision%29) (TriggeredSeconds :type Float%20%28double-precision%29) (InputAction :type Input%20Action%20Object%20Reference :default "/Game/Input/Actions/IA_Interact1.IA_Interact1"))
  (:Completed
    (if (Collision|IsOverlappingActor (Variables|Default|GetBox) (Game|Player|GetPlayerPawn 0) :!class /Script/Engine.PrimitiveComponent)
      (Class|AbilitySystemComponent|GiveAbilityandActivateOnce (Ability|GetAbilitySystemComponent (Game|GetPlayerCharacter 0)) (Variables|Default|GetAbility%20Class) 0 -1)
      (Audio|PlaySoundatLocation "/Game/Rod3nt/sounds/Ui/UI-Sound-2.UI-Sound-2" (Transformation|GetWorldLocation (Variables|Default|GetStaticMesh)) "0, 0, 0" 1.0 1.0 0.0 "/Game/Rod3nt/sounds/Concretestep1.Concretestep1" 0 0 0))))

(event EventBeginPlay
  (Input|EnableInput (Game|GetPlayerController 0))
  (bind _returnvalue (UserInterface|CreateWidget "/Game/Rod3nt/Programming/UI/WBP_RodentSwap.WBP_RodentSwap_C"))
  (Variables|Default|SetUI _returnvalue)
  (UserInterface|Viewport|AddtoViewport _returnvalue 0)
  (Variables|/Script/UMG.Widget|SetVisibility _returnvalue "Hidden"))

(fn ConstructionScript)