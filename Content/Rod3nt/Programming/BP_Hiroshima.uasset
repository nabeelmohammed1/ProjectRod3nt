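; BP_Hiroshima is a trigger actor that hides a group of static meshes and signals a sequence change when a qualifying actor enters its box.
; On box overlap, it checks that the other actor implements BI_Utli, then turns off visibility on six meshes without propagating to children.
; It then sends a fixed sequence-type value to the Game Instance through SequenceTypeMessage, with no guard against repeat triggers.
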(event OnComponentBeginOverlap(Box)
  (params (OverlappedComponent :type Primitive%20Component%20Object%20Reference) (OtherActor :type Actor%20Object%20Reference) (OtherComp :type Primitive%20Component%20Object%20Reference) (OtherBodyIndex :type Integer) (bFromSweep :type Boolean) (SweepResult :type Hit%20Result%20Structure%20%28by%20ref%29))
  (if (Utilities|DoesObjectImplementInterface OtherActor "/Game/Rod3nt/Programming/BPI+Data/BI_Utli.BI_Utli_C")
    (Rendering|SetVisibility (Variables|Default|GetStaticMesh1) false false)
    (Rendering|SetVisibility (Variables|Default|GetStaticMesh2) false false)
    (Rendering|SetVisibility (Variables|Default|GetStaticMesh3) false false)
    (Rendering|SetVisibility (Variables|Default|GetStaticMesh4) false false)
    (Rendering|SetVisibility (Variables|Default|GetStaticMesh5) false false)
    (Rendering|SetVisibility (Variables|Default|GetStaticMesh6) false false)
    (Class|BIGI|SequenceType(Message) (Game|GetGameInstance) "NewEnumerator4")))

(fn ConstructionScript)