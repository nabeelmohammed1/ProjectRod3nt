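; BP_KillGuy2 is an AI-controlled enemy character that kicks the player, playing a montage and damaging player pawn 0 directly without a hit check.
; It activates its HotMouth component shortly after BeginPlay and toggles custom depth rendering on its mesh through Turnon and TurnOff.
; CutsceneTie sets the "Stunned?" blackboard key on its controller, and GetThepath returns the first entry in AllPaths.
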(event Custom|CutsceneTie
  (AI|Components|Blackboard|SetValueasBool (AI|GetBlackboard (Pawn|GetController)) (Utilities|Name|MakeLiteralName "Stunned?") true))

(event EventBeginPlay
  (Utilities|FlowControl|Delay 2.0)
  (Components|Activation|Activate (Variables|Default|GetHotMouth) false))

(event EventTurnon
  (Rendering|SetRenderCustomDepth (Variables|Character|GetMesh) true))

(event EventTurnOff
  (Rendering|SetRenderCustomDepth (Variables|Character|GetMesh) false))

(fn ConstructionScript)

(fn AttackthePlayer
  (bind _returnvalue (Animation|PlayAnimMontage "/Game/Rod3nt/Soldiers/HumanV3/Regular/AM_Kick.AM_Kick" 1.0 "None"))
  (Game|Damage|ApplyDamage (Game|Player|GetPlayerPawn 0) 5.0 0 0)
  (return _returnvalue))

(fn GetThepath
  (return (Utilities|Array|Get(acopy) (Variables|Default|GetAll%20Paths))))