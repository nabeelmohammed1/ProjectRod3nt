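; Tank head enemy that fires BP_TankBullet from its arrow, with muzzle effect and sound, while it senses a rat player.
; AI perception tracks actors implementing BI_PLayeRat; Tick fires only when the player pawn is beyond a minimum distance, gated by a delay and timed reload.
; Custom depth toggles a highlight on the mesh.
; The Texture event marks it dead, swapping in a damaged texture and activating Niagara on the body.
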(event OnTargetPerceptionUpdated(AIPerception)
  (params (Actor :type Actor%20Object%20Reference) (Stimulus :type AI%20Stimulus%20Structure))
  (if (Utilities|DoesObjectImplementInterface Actor "/Game/Rod3nt/Programming/BPI+Data/BI_PlayeRat.BI_PLayeRat_C")
    (Variables|Default|SetSuccessfully%20Sensed (Utilities|Struct|BreakAIStimulus Stimulus))
    (Variables|Default|SetSeenActor Actor)))

(event Custom|Texture
  (bind _niagara (Variables|Default|GetNiagara))
  (bind _returnvalue (Rendering|Material|CreateDynamicMaterialInstance (Variables|Default|GetStaticMesh1) 0 "/Game/Rod3nt/MESHES/materials/MI_Tank.MI_Tank" "None" :!class /Script/Engine.PrimitiveComponent))
  (Rendering|Material|SetTextureParameterValue _returnvalue "Colour Texture" "/Game/Rod3nt/MESHES/textures/tank/sm_TankDessimated1_standardSurface2_BaseColorDAMAGED.sm_TankDessimated1_standardSurface2_BaseColorDAMAGED")
  (Class|NiagaraFunctionLibrary|OverrideSystemUserVariableStaticMeshComponent _niagara "Tank Body" (Variables|Default|GetStaticMesh1))
  (Components|Activation|Activate _niagara false)
  (Variables|Default|SetDead? true))

(event Custom|Shooting%20Reload
  (Variables|Default|Settank%20fired false)
  (Variables|Default|SetDuration 0.0)
  (Utilities|Time|ClearandInvalidateTimerbyHandle (stale EventTick _returnvalue_2)))

(event EventTurnon
  (Rendering|SetRenderCustomDepth (Variables|Default|GetStaticMesh1) true))

(event Collision|EventActorBeginOverlap
  (params (OtherActor :type Actor%20Object%20Reference)))

(event EventTick
  (params (DeltaSeconds :type Float%20%28single-precision%29))
  (bind _arrow (Variables|Default|GetArrow))
  (bind _returnvalue (Transformation|GetWorldLocation _arrow))
  (if (not (Variables|Default|GetDead?))
    (Utilities|IsValid (Variables|Default|GetSeenActor)
      (:Is%20Valid
        (if (Variables|Default|GetSuccessfully%20Sensed)
          (if (CallFunction|DistanceCheck (Game|Player|GetPlayerPawn 0))
            (if (not (Variables|Default|Gettank%20fired))
              (Utilities|FlowControl|Delay (Variables|Default|GetDuration))
              (Game|SpawnActorfromClass "/Game/Rod3nt/Programming/PICKUPSandENVI-BPS/BP_TankBullet.BP_TankBullet_C" (Math|Transform|MakeTransform _returnvalue (Transformation|GetWorldRotation _arrow) "1.000000,1.000000,1.000000") "Undefined" "MultiplyWithRoot" 0 0)
              (Niagara|SpawnSystemAttached "/Game/Rod3nt/VFX/Tank/NS_TankFiring1.NS_TankFiring1" (Variables|Default|GetArrow) "None" "0, 0, 0" "0, 0, 0" "KeepRelativeOffset" false)
              (Audio|PlaySoundatLocation "/Game/Rod3nt/sounds/tankShotCue.tankShotCue" _returnvalue "0, 0, 0" 1.0 1.0 0.0 0 0 0 0)
              (Variables|Default|Settank%20fired true)
              (bind _returnvalue_2 (Utilities|Time|SetTimerbyEvent (delegate Custom|Shooting%20Reload) 5.0))))
          (else
            (Variables|Default|SetDuration 0.2))))
      (:Is%20Not%20Valid
        (Variables|Default|SetSuccessfully%20Sensed false)
        (Variables|Default|SetSeenActor 0)))))

(event EventPlayerDied
  (Variables|Default|SetSuccessfully%20Sensed false))

(event EventTurnOff
  (Rendering|SetRenderCustomDepth (Variables|Default|GetStaticMesh1) false))

(fn ConstructionScript)

(fn DistanceCheck
  (params (Actor :type Actor%20Object%20Reference))
  (return (> (Math|Vector|Distance(Vector) (Transformation|GetActorLocation Actor) (Transformation|GetActorLocation)) 1.2e+03)))