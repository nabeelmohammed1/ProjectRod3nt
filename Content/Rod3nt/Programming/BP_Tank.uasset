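; BP_Tank is a tank whose child-actor head scans for and tracks the player rat.
; The head's AI perception flags sensed BI_PLayeRat actors, and Tick eases its yaw toward the player beyond a minimum distance.
; With nothing seen, the head rotates slowly with a turning sound.
; SendFlying wrecks the tank with an explosion, damaged textures, Niagara effect and disabled tick, while Turnon/TurnOff toggle body custom depth.
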(event Custom|PlayerSaw
  (params (Actor :type Actor%20Object%20Reference) (Stimulus :type AI%20Stimulus%20Structure))
  (if (Utilities|DoesObjectImplementInterface Actor "/Game/Rod3nt/Programming/BPI+Data/BI_PlayeRat.BI_PLayeRat_C")
    (Variables|Default|SetPlayerSeen (Utilities|Struct|BreakAIStimulus Stimulus))
    (Variables|Default|SetSeenActor Actor)))

(event EventBeginPlay
  (bind _asbp_tank_head (Utilities|Casting|CastToBP_Tank_Head (Variables|/Script/Engine.ChildActorComponent|GetChildActor (Variables|Default|GetBP_Tank_Head))))
  (EventDispatchers|BindEventtoOnTargetPerceptionUpdated (Variables|/Game/Rod3nt/Programming/BP_Tank_Head.BP_Tank_Head_C|GetAIPerception _asbp_tank_head) (delegate Custom|PlayerSaw)))

(event Collision|EventActorBeginOverlap
  (params (OtherActor :type Actor%20Object%20Reference)))

(event EventTick
  (params (DeltaSeconds :type Float%20%28single-precision%29))
  (bind _bp_tank_head (Variables|Default|GetBP_Tank_Head))
  (bind _bp_tank_head_2 (Variables|Default|GetBP_Tank_Head))
  (bind (_returnvalue _returnvalue2) (CallFunction|LookRotation _bp_tank_head _bp_tank_head))
  (bind _returnvalue_2 (Transformation|GetWorldRotation _bp_tank_head))
  (bind _returnvalue_3 (Transformation|GetWorldRotation _bp_tank_head_2))
  (if (Variables|Default|GetPlayerSeen)
    (if (CallFunction|DistanceCheck (Game|Player|GetPlayerPawn 0))
      (Utilities|IsValid (Variables|Default|GetSeenActor)
        (:Is%20Valid
          (Transformation|SetWorldRotation _bp_tank_head (Math|Rotator|MakeRotator (.roll _returnvalue_2) (.pitch _returnvalue_2) (.yaw (Math|Interpolation|RInterpTo _returnvalue _returnvalue2 DeltaSeconds 0.5))) false false))
        (:Is%20Not%20Valid
          (Variables|Default|SetPlayerSeen false)
          (Variables|Default|SetSeenActor 0))))
    (else
      (Transformation|SetWorldRotation _bp_tank_head_2 (Math|Rotator|MakeRotator (.roll _returnvalue_3) (.pitch _returnvalue_3) (+ (.yaw _returnvalue_3) (* DeltaSeconds 5.0))) false false)
      (Audio|PlaySoundatLocation "/Game/Rod3nt/sounds/TankGunRotation_Cue.TankGunRotation_Cue" (Transformation|GetWorldLocation (Variables|Default|GetDefaultSceneRoot)) "0, 0, 0" 0.1 0.9 0.0 0 0 0 0 :!label _label)
      (Utilities|FlowControl|Delay 5.0)
      (goto _label))))

(event EventPlayerDied
  (Variables|Default|SetPlayerSeen false))

(event EventSendFlying
  (params (Launch%20Vel :type Float%20%28double-precision%29))
  (bind _niagara (Variables|Default|GetNiagara))
  (Niagara|SpawnSystematLocation "/Game/Rod3nt/VFX/Explosion/NS_GrenadeExplosion.NS_GrenadeExplosion" (Transformation|GetActorLocation) "0, 0, 0" "5.000000,5.000000,5.000000")
  (Actor|Tick|SetActorTickEnabled false)
  (Components|Tick|SetComponentTickEnabled (Variables|Default|GetBP_Tank_Head) false)
  (bind _returnvalue (Rendering|Material|CreateDynamicMaterialInstance (Variables|Default|GetStaticMesh) 0 "/Game/Rod3nt/MESHES/materials/MI_Tank.MI_Tank" "None" :!class /Script/Engine.PrimitiveComponent))
  (Rendering|Material|SetTextureParameterValue _returnvalue "Colour Texture" "/Game/Rod3nt/MESHES/textures/tank/sm_TankDessimated1_standardSurface2_BaseColorDAMAGED.sm_TankDessimated1_standardSurface2_BaseColorDAMAGED")
  (Default|Texture (stale EventBeginPlay _asbp_tank_head))
  (Class|NiagaraFunctionLibrary|OverrideSystemUserVariableStaticMeshComponent _niagara "Tank Body" (Variables|Default|GetStaticMesh))
  (Components|Activation|Activate _niagara false))

(event EventTurnon
  (Rendering|SetRenderCustomDepth (Variables|Default|GetStaticMesh) true))

(event EventTurnOff
  (Rendering|SetRenderCustomDepth (Variables|Default|GetStaticMesh) false))

(event EventRecast)

(fn ConstructionScript)

(fn LookRotation
  (params (self2 :type Scene%20Component%20Object%20Reference) (self3 :type Scene%20Component%20Object%20Reference))
  (return (Transformation|GetWorldRotation self3) (Math|Rotator|FindLookatRotation (Transformation|GetWorldLocation self2) (Transformation|GetActorLocation (Game|Player|GetPlayerPawn 0)))))

(fn DistanceCheck
  (params (Actor :type Actor%20Object%20Reference))
  (return (> (Math|Vector|Distance(Vector) (Transformation|GetActorLocation Actor) (Transformation|GetWorldLocation (Variables|Default|GetBP_Tank_Head))) 1.2e+03)))

(fn AttackthePlayer
  (return 0.0))

(fn GetThepath
  (return 0))