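; BP_WindResistance is a wind volume that applies air resistance to actors implementing the BI_PLayeRat interface.
; When any actor enters the Box, it plays a 2D gust sound, before the interface check.
; Implementing actors then receive an AirResistanceMessage with the Arrow's forward vector scaled by WindStrenght, and a zero vector on exit.
; The receiver handles the effect, as the volume uses no Tick.
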(event OnComponentBeginOverlap(Box)
  (params (OverlappedComponent :type Primitive%20Component%20Object%20Reference) (OtherActor :type Actor%20Object%20Reference) (OtherComp :type Primitive%20Component%20Object%20Reference) (OtherBodyIndex :type Integer) (bFromSweep :type Boolean) (SweepResult :type Hit%20Result%20Structure%20%28by%20ref%29))
  (Audio|PlaySound2D "/Game/Rod3nt/sounds/gustOfwind_Cue.gustOfwind_Cue" 0.3 1.0 0.0 0 0)
  (if (Utilities|DoesObjectImplementInterface OtherActor "/Game/Rod3nt/Programming/BPI+Data/BI_PlayeRat.BI_PLayeRat_C")
    (Class|BIPLayeRat|AirResistance(Message) OtherActor (* (Math|Vector|GetForwardVector (Variables|Default|GetArrow)) (Variables|Default|GetWindStrenght')))))

(event OnComponentEndOverlap(Box)
  (params (OverlappedComponent :type Primitive%20Component%20Object%20Reference) (OtherActor :type Actor%20Object%20Reference) (OtherComp :type Primitive%20Component%20Object%20Reference) (OtherBodyIndex :type Integer))
  (if (Utilities|DoesObjectImplementInterface OtherActor "/Game/Rod3nt/Programming/BPI+Data/BI_PlayeRat.BI_PLayeRat_C")
    (Class|BIPLayeRat|AirResistance(Message) OtherActor "0, 0, 0")))

(event EventBeginPlay)

(event Collision|EventActorBeginOverlap
  (params (OtherActor :type Actor%20Object%20Reference)))

(event EventTick
  (params (DeltaSeconds :type Float%20%28single-precision%29)))

(fn ConstructionScript)