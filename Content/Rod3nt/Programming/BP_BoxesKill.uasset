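; Trigger actor that hides four static meshes and starts a cutscene step, apparently a box-based kill involving a boss.
; The BossCheck volume enables Box query collision while an actor tagged "Boss" overlaps it and disables it on exit.
; Any Box overlap hides the meshes.
; If the overlapping actor implements BI_Utli, it also sends a sequence type to the GameInstance and calls CutsceneTie on BP_KillGuy2.
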(event OnComponentBeginOverlap(Box)
  (params (OverlappedComponent :type Primitive%20Component%20Object%20Reference) (OtherActor :type Actor%20Object%20Reference) (OtherComp :type Primitive%20Component%20Object%20Reference) (OtherBodyIndex :type Integer) (bFromSweep :type Boolean) (SweepResult :type Hit%20Result%20Structure%20%28by%20ref%29))
  (Rendering|SetVisibility (Variables|Default|GetStaticMesh1) false false)
  (Rendering|SetVisibility (Variables|Default|GetStaticMesh2) false false)
  (Rendering|SetVisibility (Variables|Default|GetStaticMesh3) false false)
  (Rendering|SetVisibility (Variables|Default|GetStaticMesh4) false false)
  (if (Utilities|DoesObjectImplementInterface OtherActor "/Game/Rod3nt/Programming/BPI+Data/BI_Utli.BI_Utli_C")
    (Class|BIGI|SequenceType(Message) (Game|GetGameInstance) "NewEnumerator7")
    (bind _returnvalue (Actor|GetActorOfClass "/Game/Rod3nt/Programming/BP_KillGuy2.BP_KillGuy2_C"))
    (Default|CutsceneTie _returnvalue)))

(event OnComponentBeginOverlap(BossCheck)
  (params (OverlappedComponent :type Primitive%20Component%20Object%20Reference) (OtherActor :type Actor%20Object%20Reference) (OtherComp :type Primitive%20Component%20Object%20Reference) (OtherBodyIndex :type Integer) (bFromSweep :type Boolean) (SweepResult :type Hit%20Result%20Structure%20%28by%20ref%29))
  (if (Actor|ActorHasTag OtherActor "Boss")
    (Collision|SetCollisionEnabled (Variables|Default|GetBox) "QueryOnly")))

(event OnComponentEndOverlap(BossCheck)
  (params (OverlappedComponent :type Primitive%20Component%20Object%20Reference) (OtherActor :type Actor%20Object%20Reference) (OtherComp :type Primitive%20Component%20Object%20Reference) (OtherBodyIndex :type Integer))
  (if (Actor|ActorHasTag OtherActor "Boss")
    (Collision|SetCollisionEnabled (Variables|Default|GetBox) "NoCollision")))

(fn ConstructionScript)