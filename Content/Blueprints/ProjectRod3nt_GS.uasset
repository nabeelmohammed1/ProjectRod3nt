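; ProjectRod3nt_GS is a global hub of events for audio, sequences and achievements, apparently the game state going by its name.
; It stores and applies master volume through a sound mix override, and sets that base mix shortly after initialization.
; Sequence and tutorial cutscene events relay to dispatchers, while another event stores sequencer death triggers.
; Achievement events cache achievements for the first player, then write progress by name.
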(event Custom|VolumeChange
  (params (Volume :type Float%20%28double-precision%29))
  (Variables|Default|SetVolume Volume)
  (Audio|SetSoundMixClassOverride "/Game/Blueprints/ProjectRod3ntSoundMix.ProjectRod3ntSoundMix" "/Engine/EngineSounds/Master.Master" (Variables|Default|GetVolume) 1.0 1.0 true))

(event Custom|Call%20To%20Level
  (params (SequencerDeathTriggers :type EDeathSequence%20Enum :default "NewEnumerator0"))
  (Variables|Default|SetSequencerDeathTriggers SequencerDeathTriggers))

(event EventSequenceType
  (params (Sequence :type EDeathSequence%20Enum :default "NewEnumerator0"))
  (Default|CallCalltoLvl Sequence))

(event EventTutorialEvent
  (Default|CallTutorialCutscene))

(event EventInit
  (Utilities|FlowControl|Delay 0.2)
  (Class|GameplayStatics|SetBaseSoundMix "/Game/Blueprints/ProjectRod3ntSoundMix.ProjectRod3ntSoundMix"))

(event EventAchievmentType
  (params (Name :type String) (Level :type Float%20%28double-precision%29))
  (bind _returnvalue (Game|GetPlayerController 0))
  (|CacheAchievements _returnvalue
    (:OnSuccess
      (|WriteProgress _returnvalue Name Level))))

(fn TheCurrentArray
  (return 0))